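; BP_DayNightBox is a placed sphere volume that shifts sun, skylight, height fog and sky dome toward its own look as the player enters.
; While the pawn overlaps, Tick blends GS_Skylands defaults to target values by horizontal camera distance across TransitionRadius, updating again on exit.
; The construction script previews the target sun, and its PopulateData toggle snapshots targets from level actors.
; Skylight intensity blends from DefaultSunIntensity, and a debug print remains.
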(event OnComponentBeginOverlap(Collision)
  (params (OverlappedComponent :type Primitive%20Component%20Object%20Reference) (OtherActor :type Actor%20Object%20Reference) (OtherComp :type Primitive%20Component%20Object%20Reference) (OtherBodyIndex :type Integer) (bFromSweep :type Boolean) (SweepResult :type Hit%20Result%20Structure%20%28by%20ref%29))
  ;[1 1 1] Checks if your character has entered the Collision Box
  (if (== OtherActor (Game|Player|GetPlayerPawn 0))
    (Variables|Default|SetInRange true)))

(event OnComponentEndOverlap(Collision)
  (params (OverlappedComponent :type Primitive%20Component%20Object%20Reference) (OtherActor :type Actor%20Object%20Reference) (OtherComp :type Primitive%20Component%20Object%20Reference) (OtherBodyIndex :type Integer))
  (bind _returnvalue (Game|GetPlayerController 0))
  (bind _transitionradius (Variables|Default|GetTransitionRadius))
  (bind _collision (Variables|Default|GetCollision))
  (bind _sphereradius (Variables|Default|GetSphereRadius))
  (bind _returnvalue_2 (Transformation|GetWorldLocation _collision))
  (bind _returnvalue_3 (- _sphereradius _transitionradius))
  (bind _playercameramanager (Variables|/Script/Engine.PlayerController|GetPlayerCameraManager _returnvalue))
  (bind _returnvalue_4 (Camera|GetCameraLocation _playercameramanager))
  (bind _returnvalue_5 (- _returnvalue_4 _returnvalue_2))
  (bind _returnvalue_6 (Math|Vector|VectorLengthXY _returnvalue_5))
  (bind _returnvalue_7 (Math|Float|NormalizetoRange _returnvalue_6 _returnvalue_3 _sphereradius))
  (bind _returnvalue_8 (Math|Float|Clamp(Float) _returnvalue_7))
  (bind _returnvalue_9 (- 1.0 _returnvalue_8))
  ;[1 1 1] Checks if your character has entered the Collision Box
  (if (== OtherActor (Game|Player|GetPlayerPawn 0))
    (Variables|Default|SetInRange false)
    ;[1 1 1] Sun Angle
    (Sun|SetSunAngle (Math|Rotator|Lerp(Rotator) (References|GetDefaultSunAngle) (Variables|Sun|GetTargetSunAngle) _returnvalue_9 true))
    ;[1 1 1] Sun Brightness
    (Sun|SetSunIntensity (Math|Float|Lerp (Variables|/Game/TwentyItems/Blueprints/Main/Skylands/GS_Skylands.GS_Skylands_C|GetDefaultSunIntensity (References|GetGameStateRef)) (Variables|Sun|GetTargetSunIntensity) _returnvalue_9))
    (Skylight|UpdateSkyLight _returnvalue_9)
    (Fog|UpdateExponentialHeightFog _returnvalue_9)
    (Sky|UpdateSky _returnvalue_9)))

(event EventBeginPlay
  ;[1 0 0] Event Begin Play
  (References|GetSkyReferences))

(event EventTick
  (params (DeltaSeconds :type Float%20%28single-precision%29))
  (bind _returnvalue (Game|GetPlayerController 0))
  (bind _transitionradius (Variables|Default|GetTransitionRadius))
  (bind _collision (Variables|Default|GetCollision))
  (bind _sphereradius (Variables|Default|GetSphereRadius))
  (bind _returnvalue_2 (Transformation|GetWorldLocation _collision))
  (bind _returnvalue_3 (- _sphereradius _transitionradius))
  (bind _playercameramanager (Variables|/Script/Engine.PlayerController|GetPlayerCameraManager _returnvalue))
  (bind _returnvalue_4 (Camera|GetCameraLocation _playercameramanager))
  (bind _returnvalue_5 (- _returnvalue_4 _returnvalue_2))
  (bind _returnvalue_6 (Math|Vector|VectorLengthXY _returnvalue_5))
  (bind _returnvalue_7 (Math|Float|NormalizetoRange _returnvalue_6 _returnvalue_3 _sphereradius))
  (bind _returnvalue_8 (Math|Float|Clamp(Float) _returnvalue_7))
  (bind _returnvalue_9 (- 1.0 _returnvalue_8))
  (if (CallFunction|PlayerinRange?)
    ;[1 1 1] Sun Angle
    (Sun|SetSunAngle (Math|Rotator|Lerp(Rotator) (References|GetDefaultSunAngle) (Variables|Sun|GetTargetSunAngle) _returnvalue_9 true))
    ;[1 1 1] Sun Brightness
    (Sun|SetSunIntensity (Math|Float|Lerp (Variables|/Game/TwentyItems/Blueprints/Main/Skylands/GS_Skylands.GS_Skylands_C|GetDefaultSunIntensity (References|GetGameStateRef)) (Variables|Sun|GetTargetSunIntensity) _returnvalue_9))
    (Skylight|UpdateSkyLight _returnvalue_9)
    (Fog|UpdateExponentialHeightFog _returnvalue_9)
    (Sky|UpdateSky _returnvalue_9)))

(fn ConstructionScript
  (Utilities|FlowControl|Sequence
    (:then_0
      (if (and (Utilities|IsValid (Variables|References|GetSun)) (Utilities|IsValid (Variables|References|GetSkyDome)))
        (Transformation|SetActorRotation (Variables|References|GetSun) (Variables|Sun|GetTargetSunAngle))
        (Default|UpdateSunDirection (Variables|References|GetSkyDome))
        (Sun|SetSunIntensity (Variables|Sun|GetTargetSunIntensity))))
    (:then_1
      (Components|Sphere|SetSphereRadius (Variables|Default|GetCollision) (Variables|Default|GetSphereRadius) true))
    (:then_2
      (if (Variables|Default|GetPopulateData)
        (Fog|PopulateFogData)
        (CallFunction|PopulateSunData)
        (Skylight|PopulateSkyLightData)
        (Sky|PopulateSkyData)
        (Variables|Default|SetPopulateData false)))))

(fn SetSunAngle
  (params (New%20Angle :type Rotator))
  (bind _sun (Variables|References|GetSun))
  (bind _skydome (Variables|References|GetSkyDome))
  (Variables|Sun|SetCurrentSunAngle New%20Angle)
  (Utilities|IsValid _sun
    (:Is%20Valid
      (Transformation|SetActorRotation _sun New%20Angle)
      (Utilities|IsValid _skydome
        (:Is%20Valid
          (Default|UpdateSunDirection _skydome))))))

(fn GetSkyReferences
  (bind _gs_expresslane (References|GetGameStateRef))
  (Utilities|FlowControl|Sequence
    (:then_0
      ;[1 1 1] Gets References To the sky sphere and sun light if they aren't set in the level editor
      (Variables|References|SetSkyDome (Variables|/Game/TwentyItems/Blueprints/Main/Skylands/GS_Skylands.GS_Skylands_C|GetSkySphereRef _gs_expresslane)))
    (:then_1
      (Variables|References|SetSun (Variables|/Game/TwentyItems/Blueprints/Main/Skylands/GS_Skylands.GS_Skylands_C|GetDirectionalLightRef _gs_expresslane)))
    (:then_2
      (Variables|References|SetExponentialHeightFogRef (Variables|/Game/TwentyItems/Blueprints/Main/Skylands/GS_Skylands.GS_Skylands_C|GetVolumetricFogReference _gs_expresslane)))
    (:then_3
      (Variables|References|SetSkyLightRef (Variables|/Game/TwentyItems/Blueprints/Main/Skylands/GS_Skylands.GS_Skylands_C|GetSkyLightRef _gs_expresslane)))))

(fn GetGameStateRef
  (Utilities|IsValid (Variables|References|GetGS_Skylands)
    (:Is%20Valid
      _)
    (:Is%20Not%20Valid
      (bind _output_get (Variables|References|SetGS_Skylands (.AsGS%20Skylands (Utilities|Casting|CastToGS_Skylands (Game|GetGameState)))))))
  (return _output_get))

(fn GetDefaultSunAngle
  (return (Variables|/Game/TwentyItems/Blueprints/Main/Skylands/GS_Skylands.GS_Skylands_C|GetDefaultSunPosition (References|GetGameStateRef))))

(fn UpdateExponentialHeightFog
  (params (Alpha :type Float%20%28single-precision%29%20%28by%20ref%29))
  (bind _gs_expresslane (References|GetGameStateRef))
  (bind _exponentialheightfogref (Variables|References|GetExponentialHeightFogRef))
  (bind _fogdata (Variables|Fog|GetFogData))
  (bind (_fogdensity _foginscatteringcolor _fogheightfalloff _fogmaxopacity _startdistance _fogcutoffdistance _volumetricfog _scatteringdistribution _extinctionscale _viewdistance) (Utilities|Struct|BreakFogStruct _fogdata))
  (bind _component (Variables|/Script/Engine.ExponentialHeightFog|GetComponent _exponentialheightfogref))
  (bind _defaultfogparameters (Variables|/Game/TwentyItems/Blueprints/Main/Skylands/GS_Skylands.GS_Skylands_C|GetDefaultFogParameters _gs_expresslane))
  (bind (_fogdensity_2 _foginscatteringcolor_2 _fogheightfalloff_2 _fogmaxopacity_2 _startdistance_2 _fogcutoffdistance_2 _volumetricfog_2 _scatteringdistribution_2 _extinctionscale_2 _viewdistance_2) (Utilities|Struct|BreakFogStruct _defaultfogparameters))
  (Utilities|IsValid _exponentialheightfogref
    (:Is%20Valid
      (Class|ExponentialHeightFogComponent|SetFogDensity _component (Math|Float|Lerp _fogdensity_2 _fogdensity Alpha))
      (Class|ExponentialHeightFogComponent|SetFogInscatteringColor _component (Math|Color|Lerp(LinearColor) _foginscatteringcolor_2 _foginscatteringcolor Alpha))
      (Class|ExponentialHeightFogComponent|SetFogHeightFalloff _component (Math|Float|Lerp _fogheightfalloff_2 _fogheightfalloff Alpha))
      (Class|ExponentialHeightFogComponent|SetFogMaxOpacity _component (Math|Float|Lerp _fogmaxopacity_2 _fogmaxopacity Alpha))
      (Class|ExponentialHeightFogComponent|SetStartDistance _component (Math|Float|Lerp _startdistance_2 _startdistance Alpha))
      (Class|ExponentialHeightFogComponent|SetFogCutoffDistance _component (Math|Float|Lerp _fogcutoffdistance_2 _fogcutoffdistance Alpha))
      (Class|ExponentialHeightFogComponent|SetVolumetricFog _component (select (>= Alpha 0.5) _volumetricfog _volumetricfog_2))
      (Class|ExponentialHeightFogComponent|SetVolumetricFogScatteringDistribution _component (Math|Float|Lerp _scatteringdistribution_2 _scatteringdistribution Alpha))
      (Class|ExponentialHeightFogComponent|SetVolumetricFogExtinctionScale _component (Math|Float|Lerp _extinctionscale_2 _extinctionscale Alpha))
      (Class|ExponentialHeightFogComponent|SetVolumetricFogDistance _component (Math|Float|Lerp _viewdistance_2 _viewdistance Alpha)))))

(fn PopulateFogData
  (bind _outactors (Actor|GetAllActorsOfClass "/Script/Engine.ExponentialHeightFog"))
  (Utilities|IsValid (Utilities|Array|Get(acopy) _outactors)
    (:Is%20Valid
      (Utilities|Struct|SetmembersinFogStruct (Variables|Fog|GetFogData) (Variables|/Script/Engine.ExponentialHeightFogComponent|GetFogDensity (Variables|/Script/Engine.ExponentialHeightFog|GetComponent (Utilities|Array|Get(acopy) _outactors))) (Variables|/Script/Engine.ExponentialHeightFogComponent|GetFogInscatteringColor (Variables|/Script/Engine.ExponentialHeightFog|GetComponent (Utilities|Array|Get(acopy) _outactors))) (Variables|/Script/Engine.ExponentialHeightFogComponent|GetFogHeightFalloff (Variables|/Script/Engine.ExponentialHeightFog|GetComponent (Utilities|Array|Get(acopy) _outactors))) (Variables|/Script/Engine.ExponentialHeightFogComponent|GetFogMaxOpacity (Variables|/Script/Engine.ExponentialHeightFog|GetComponent (Utilities|Array|Get(acopy) _outactors))) (Variables|/Script/Engine.ExponentialHeightFogComponent|GetStartDistance (Variables|/Script/Engine.ExponentialHeightFog|GetComponent (Utilities|Array|Get(acopy) _outactors))) (Variables|/Script/Engine.ExponentialHeightFogComponent|GetFogCutoffDistance (Variables|/Script/Engine.ExponentialHeightFog|GetComponent (Utilities|Array|Get(acopy) _outactors))) (Variables|/Script/Engine.ExponentialHeightFogComponent|GetbEnableVolumetricFog (Variables|/Script/Engine.ExponentialHeightFog|GetComponent (Utilities|Array|Get(acopy) _outactors))) (Variables|/Script/Engine.ExponentialHeightFogComponent|GetVolumetricFogScatteringDistribution (Variables|/Script/Engine.ExponentialHeightFog|GetComponent (Utilities|Array|Get(acopy) _outactors))) (Variables|/Script/Engine.ExponentialHeightFogComponent|GetVolumetricFogExtinctionScale (Variables|/Script/Engine.ExponentialHeightFog|GetComponent (Utilities|Array|Get(acopy) _outactors))) (Variables|/Script/Engine.ExponentialHeightFogComponent|GetVolumetricFogDistance (Variables|/Script/Engine.ExponentialHeightFog|GetComponent (Utilities|Array|Get(acopy) _outactors)))))))

(fn SetSunIntensity
  (params (New%20Intensity :type Float%20%28single-precision%29))
  (bind _sun (Variables|References|GetSun))
  (bind _output_get (Variables|Sun|SetCurrentSunIntensity New%20Intensity))
  (Utilities|IsValid _sun
    (:Is%20Valid
      (Rendering|Components|Light|SetIntensity (Variables|/Script/Engine.Light|GetLightComponent _sun) _output_get))))

(fn UpdateSkyLight
  (params (Alpha :type Float%20%28single-precision%29))
  (bind _gs_expresslane (References|GetGameStateRef))
  (bind _skylightcubemap (Variables|SkyLight|GetSkyLightCubeMap))
  (bind _skylightref (Variables|References|GetSkyLightRef))
  (bind _lightcomponent (Variables|/Script/Engine.SkyLight|GetLightComponent _skylightref))
  (Utilities|IsValid _skylightref
    (:Is%20Valid
      (Rendering|Components|Light|SetIntensity _lightcomponent (Math|Float|Lerp (Variables|/Game/TwentyItems/Blueprints/Main/Skylands/GS_Skylands.GS_Skylands_C|GetDefaultSunIntensity _gs_expresslane) (Variables|SkyLight|GetTargetSkyLightIntensity) Alpha))
      (Class|SkyLightComponent|SetCubemapBlend _lightcomponent (Variables|/Game/TwentyItems/Blueprints/Main/Skylands/GS_Skylands.GS_Skylands_C|GetDefaultSkyLightCubeMap _gs_expresslane) _skylightcubemap Alpha)
      (Development|PrintString (Utilities|GetDisplayName _skylightcubemap) true true "(R=0.344412,G=1.000000,B=0.515343,A=1.000000)" 0.0))))

(fn PlayerinRange?
  (return (Utilities|Array|ContainsItem (Collision|GetOverlappingActors (Variables|Default|GetCollision) "/Script/Engine.Pawn" :!class /Script/Engine.PrimitiveComponent) (Game|Player|GetPlayerPawn 0))))

(fn Distance
  (params (Location :type Vector)))

(fn PopulateSunData
  (bind _outactors (Actor|GetAllActorsOfClass "/Script/Engine.DirectionalLight"))
  (Variables|Sun|SetTargetSunIntensity (Variables|/Script/Engine.LightComponentBase|GetIntensity (Variables|/Script/Engine.Light|GetLightComponent (Utilities|Array|Get(acopy) _outactors))))
  (Variables|Sun|SetTargetSunAngle (Transformation|GetActorRotation (Utilities|Array|Get(acopy) _outactors))))

(fn PopulateSkyLightData
  (bind _outactors (Actor|GetAllActorsOfClass "/Script/Engine.SkyLight"))
  (Variables|SkyLight|SetTargetSkyLightIntensity (Variables|/Script/Engine.LightComponentBase|GetIntensity (Variables|/Script/Engine.SkyLight|GetLightComponent (Utilities|Array|Get(acopy) _outactors))))
  (Variables|SkyLight|SetSkyLightCubeMap (Variables|/Script/Engine.SkyLightComponent|GetCubemap (Variables|/Script/Engine.SkyLight|GetLightComponent (Utilities|Array|Get(acopy) _outactors)))))

(fn UpdateSky
  (params (Alpha :type Float%20%28single-precision%29))
  (bind _gs_expresslane (References|GetGameStateRef))
  (bind _skydome (Variables|References|GetSkyDome))
  (Variables|/Engine/EngineSky/BP_Sky_Sphere.BP_Sky_Sphere_C|SetCloud%20opacity _skydome (Math|Float|Lerp (Variables|/Game/TwentyItems/Blueprints/Main/Skylands/GS_Skylands.GS_Skylands_C|GetDefaultCloudOpacity _gs_expresslane) (Variables|SkyData|GetTargetCloudOpacity) Alpha))
  (Variables|/Engine/EngineSky/BP_Sky_Sphere.BP_Sky_Sphere_C|SetCloud%20speed _skydome (Math|Float|Lerp (Variables|/Game/TwentyItems/Blueprints/Main/Skylands/GS_Skylands.GS_Skylands_C|GetDefaultCloudSpeed _gs_expresslane) (Variables|SkyData|GetTargetCloudSpeed) Alpha))
  (Variables|/Engine/EngineSky/BP_Sky_Sphere.BP_Sky_Sphere_C|SetStars%20brightness _skydome (Math|Float|Lerp (Variables|/Game/TwentyItems/Blueprints/Main/Skylands/GS_Skylands.GS_Skylands_C|GetDefaultStarBrightness _gs_expresslane) (Variables|SkyData|GetTargetStarBrightness) Alpha))
  (Default|RefreshMaterial (Variables|References|GetSkyDome)))

(fn PopulateSkyData
  (bind _outactors (Actor|GetAllActorsOfClass "/Engine/EngineSky/BP_Sky_Sphere.BP_Sky_Sphere_C"))
  (Variables|SkyData|SetTargetCloudOpacity (Variables|/Engine/EngineSky/BP_Sky_Sphere.BP_Sky_Sphere_C|GetCloud%20opacity (Utilities|Array|Get(acopy) _outactors)))
  (Variables|SkyData|SetTargetCloudSpeed (Variables|/Engine/EngineSky/BP_Sky_Sphere.BP_Sky_Sphere_C|GetCloud%20speed (Utilities|Array|Get(acopy) _outactors)))
  (Variables|SkyData|SetTargetStarBrightness (Variables|/Engine/EngineSky/BP_Sky_Sphere.BP_Sky_Sphere_C|GetStars%20brightness (Utilities|Array|Get(acopy) _outactors))))