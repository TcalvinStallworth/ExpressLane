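; Older Express Lane game mode that runs a team match through lobby, countdown, preparation, lights-out, overtime and end-game phases.
; Timers drive the phase changes, mirroring state to the GameState and steering the day/night cycle.
; Lobby joins spawn at random capsule-checked starts, while bombay creation is delegated to the ProceduralLevelManager.
; Bombay respawn, bombay destruction and death/elimination handling are stubbed or disconnected.
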(event Custom|GetLobbySpawnPoints
  ;[1 1 1] Gets Lobby Spawn Points
  (bind _outactors (Actor|GetAllActorsOfClass "/Game/TwentyItems/Blueprints/Main/Spawning/LobbyPlayerStart.LobbyPlayerStart_C"))
  (Variables|LobbySpawning|SetLobbySpawnPoints _outactors)
  ;;[1 1 1] Sets Regestered Spawn Points to true
  (Variables|LobbySpawning|SetRegisteredSpawnPoints? true)
  ;;[1 1 1] Spawns Loaded in Players
  (for _array_element (Variables|/Script/Engine.GameStateBase|GetPlayerArray (Game|GetGameState))
    (bind _asplayer_controller (Utilities|Casting|CastToPlayerController (Components|GetOwner _array_element)))
    (Spawning|SpawnPlayer _asplayer_controller)))

(event EventBeginPlay
  ;[1 1 1] Event Begin Play
  (Networking|SwitchHasAuthority
    (:Authority
      (CallFunction|GetLobbySpawnPoints)
      (CallFunction|StartWaitingforPlayersState))))

(event EventOnLogout
  (params (ExitingController :type Controller%20Object%20Reference))
  ;[1 1 1] Event On Logout
  (Players|PlayLeftGame ExitingController)
  (Players|PlayLeftGame ExitingController))

(event EventPostLogin
  (params (NewPlayer :type Player%20Controller%20Object%20Reference))
  ;[1 1 1] Event Post Login Lobby
  (Spawning|SpawnPlayer NewPlayer)
  (Players|PlayerJoinedGame NewPlayer))

(event Custom|StartWaitingForPlayersState
  ;[1 0 0] Start Waiting For Players State
  (MatchState|StartWaitingforPlayers))

(event Custom|PrepareToStartGame
  ;[1 0 0] Starts CountDown To Begin Game and spawns the bombays
  (MatchState|PreparetoStartGameFunction))

(event Custom|StartGame
  ;[1 0 0] Start Game
  (MatchState|StartGameFunction))

(event Custom|LightsOut
  ;[1 0 0] Lights Out
  (MatchState|LightsOutFunction))

(event Custom|LightsOnCountdown
  ;[1 0 0] Lights On CountDown
  (MatchState|LightsonCountDownFunction))

(event Custom|StartOvertimePhase
  ;[1 0 0] Start OverTime Phase
  (MatchState|StartOverTimePhaseFunction))

(event Custom|EndGame
  ;[1 0 0] Game is Over
  (MatchState|EndGameFunction))

(fn ConstructionScript)

(fn GetPickUpTallies
  (bind (_data _foundrow) (CallFunction|GetSpawnableLootfromDataTable "ShelfLoot"))
  (Networking|SwitchHasAuthority
    (:Authority
      ;[1 1 1] Checks if Pickup spawners were already tallied
      (if (not (Variables|PickupSpawners|GetTalliedPickUpSpawners?))
        (if _foundrow
          ;[1 1 1] Adds up all the pickup spawn rates to get the max int to randomize when spawning a pickup
          (for _array_element (.Loot (Utilities|Struct|BreakSpawnableLootStruct _data))
            (Variables|PickupSpawners|SetPickUpSpawnerTotalTallies (+ (.SpawnRate (Utilities|Struct|BreakLootable_Struct _array_element)) (Variables|PickupSpawners|GetPickUpSpawnerTotalTallies))))
          (Variables|PickupSpawners|SetTalliedPickUpSpawners? true)))
      (return (Variables|PickupSpawners|GetPickUpSpawnerTotalTallies)))))

(fn SpawnBombays
  (bind _outactors (Actor|GetAllActorsOfClass "/Game/TwentyItems/Blueprints/ProceduralGeneration/ProceduralLevelManager.ProceduralLevelManager_C"))
  (bind _output_get (Variables|Territory|SetProceduralLevelManager (Utilities|Array|Get(acopy) _outactors)))
  (Default|CreateBombaySpawnPoints _output_get))

(fn GetBombaySpawnPoints)

(fn GetGameStateReference
  (bind _asgs_express_lane_old (Utilities|Casting|CastToGS_ExpressLaneOLD (Game|GetGameState)))
  (return _asgs_express_lane_old))

(fn SpawnPlayersonMatchBegin
  ;[1 1 1] Tells every team to spawn their players at their bombay
  (for _array_element (Variables|/Game/TwentyItems/Blueprints/Main/GS_ExpressLaneOLD.GS_ExpressLaneOLD_C|GetTeams (References|GetGameStateReference))
    (LocalVariables|SetCurrentTeam _array_element)))

(fn SpawnPlayer
  (params (Player%20Controller :type Player%20Controller%20Object%20Reference))
  (bind _lobbyspawnpoints (Variables|LobbySpawning|GetLobbySpawnPoints))
  (LocalVariables|SetSpawningPC Player%20Controller)
  ;[1 1 1] Checks if the match has started
  (if (not (Variables|MatchState|GetMatchStarted?))
    ;[1 1 1] Match Hasn't Started
    ;;[1 1 1] Checks if the lobby spawn points have been registered
    (if (Variables|LobbySpawning|GetRegisteredSpawnPoints?)
      ;;[1 1 1] Destroys Current Controlled Pawn
      (Utilities|IsValid (Pawn|GetControlledPawn (LocalVariables|GetSpawningPC))
        (:Is%20Valid
          (Actor|DestroyActor (Pawn|GetControlledPawn (LocalVariables|GetSpawningPC))))
        (:Is%20Not%20Valid
          _))
      ;;[1 1 1] Selects random spawn point to spawn player at
      (bind _output_get (LocalVariables|SetSpawnIndex (Math|Random|RandomIntegerinRange 0 (Utilities|Array|LastIndex _lobbyspawnpoints)) :!label _label))
      ;;[1 1 1] Checks if there is currently a player standing in the location selected for spawn
      (bind _returnvalue (Class|KismetSystemLibrary|CapsuleTraceSingleforObjects (Transformation|GetWorldLocation (Variables|/Game/TwentyItems/Blueprints/Main/Spawning/LobbyPlayerStart.LobbyPlayerStart_C|GetCapsule (Utilities|Array|Get(acopy) _lobbyspawnpoints _output_get))) (Transformation|GetWorldLocation (Variables|/Game/TwentyItems/Blueprints/Main/Spawning/LobbyPlayerStart.LobbyPlayerStart_C|GetCapsule (Utilities|Array|Get(acopy) _lobbyspawnpoints _output_get))) (Components|Capsule|GetScaledCapsuleRadius (Variables|/Game/TwentyItems/Blueprints/Main/Spawning/LobbyPlayerStart.LobbyPlayerStart_C|GetCapsule (Utilities|Array|Get(acopy) _lobbyspawnpoints _output_get))) (Components|Capsule|GetScaledCapsuleHalfHeight (Variables|/Game/TwentyItems/Blueprints/Main/Spawning/LobbyPlayerStart.LobbyPlayerStart_C|GetCapsule (Utilities|Array|Get(acopy) _lobbyspawnpoints _output_get))) (Utilities|Array|MakeArray "ObjectTypeQuery3") false 0 "None" true))
      (if (not _returnvalue)
        _
        (else
          ;;[1 1 1] Prevents Infinite Loops
          (bind _output_get_2 (LocalVariables|SetSpawnAttempts (+ (LocalVariables|GetSpawnAttempts) 1)))
          (if (>= _output_get_2 (Utilities|Array|Length (Variables|LobbySpawning|GetLobbySpawnPoints)))
            _
            (else
              (goto _label)))))
      ;;[1 1 1] Spawns and possessescharacter at randomly selected lobby spawn point
      (bind _returnvalue_2 (Game|SpawnActorfromClass "/Game/TwentyItems/Blueprints/Player/ExpressLaneCharacter.ExpressLaneCharacter_C" (Math|Transform|MakeTransform (.location (Transformation|GetActorTransform (Utilities|Array|Get(acopy) (Variables|LobbySpawning|GetLobbySpawnPoints) (LocalVariables|GetSpawnIndex)))) (.rotation (Transformation|GetActorTransform (Utilities|Array|Get(acopy) (Variables|LobbySpawning|GetLobbySpawnPoints) (LocalVariables|GetSpawnIndex)))) (.scale (Transformation|GetActorTransform (Utilities|Array|Get(acopy) (Variables|LobbySpawning|GetLobbySpawnPoints) (LocalVariables|GetSpawnIndex))))) "AdjustIfPossibleButAlwaysSpawn" (LocalVariables|GetSpawningPC) "0.000000,0.000000,0.000000" 0 0))
      (Pawn|Possess (LocalVariables|GetSpawningPC) _returnvalue_2))))

(fn LobbyStartTimer
  ;[1 1 1] Counts Down Every Second
  (bind _output_get (Variables|MatchState|SetLobbyTimeCountDown (- (Variables|MatchState|GetLobbyTimeCountDown) 1.0)))
  (if (or (< _output_get 1.0) (> (Utilities|Array|Length (Variables|/Script/Engine.GameStateBase|GetPlayerArray (References|GetGameStateReference))) (Variables|MatchState|GetPlayersToStartGame)))
    ;[1 1 1] Prepares To Start Game
    (CallFunction|PreparetoStartGame)
    ;[1 1 1] Clears Timer Handle
    (Utilities|Time|ClearandInvalidateTimerbyHandle (Variables|MatchState|GetLobbyStartTimerHandle))))

(fn StartGameTimer
  ;[1 1 1] Updates Time left before starting match
  (bind _output_get (Variables|MatchState|SetTimeLeftToStartMatch (- (Variables|MatchState|GetTimeLeftToStartMatch) 1)))
  ;[1 1 1] Updates for Clients
  (Variables|/Game/TwentyItems/Blueprints/Main/GS_ExpressLaneOLD.GS_ExpressLaneOLD_C|SetTimeUntilGameStarts (References|GetGameStateReference) _output_get)
  ;[1 1 1] Checks if the match is ready to start
  (if (<= (Variables|MatchState|GetTimeLeftToStartMatch) 0)
    ;[1 1 1] Starts Game
    (CallFunction|StartGame)
    ;[1 1 1] Clears Timer
    (Utilities|Time|ClearandInvalidateTimerbyHandle (Variables|MatchState|GetGameStartTimerHandle))))

(fn SetLightsOutTimer
  (bind _lightsoutrange (Variables|MatchStateParameters|GetLightsOutRange))
  (bind (_x _y) (Math|Vector2D|BreakVector2D _lightsoutrange))
  (Variables|MatchState|SetLightsOutTime (Math|Random|RandomIntegerinRange (Math|Float|Round _x) (Math|Float|Round _y)))
  (bind _returnvalue (Utilities|Time|SetTimerbyFunctionName 0 "LightsOutTimer" 1.0 true))
  (Variables|MatchState|SetLightsOutTimerHandle _returnvalue))

(fn LightsOutTimer
  (bind _output_get (Variables|MatchState|SetLightsOutTimeElapsed (+ (Variables|MatchState|GetLightsOutTimeElapsed) 1)))
  (if (>= _output_get (Variables|MatchState|GetLightsOutTime))
    (Utilities|Time|ClearandInvalidateTimerbyHandle (Variables|MatchState|GetLightsOutTimerHandle))
    (CallFunction|LightsOut)))

(fn AttemptSetUpShelves
  (if (and (Variables|PickUps|GetReadyToSpawnChests?) (Variables|PickUps|GetReadyToSpawnPickups?))
    (for _array_element (Variables|Shelves|GetSpawnedShelves)
      (Default|BeginSpawningShelves _array_element))))

(fn PlayerJoinedGame
  (params (Player%20Controller :type Player%20Controller%20Object%20Reference))
  (Utilities|Array|Add (Variables|Players|GetPlayersInGame) Player%20Controller))

(fn PlayLeftGame
  (params (Controller :type Controller%20Object%20Reference))
  (Utilities|Array|RemoveItem (Variables|Players|GetPlayersInGame) Controller))

(fn GetProceduralLevelManagerRef
  (Utilities|IsValid (Variables|Territory|GetProceduralLevelManager)
    (:Is%20Valid
      _)
    (:Is%20Not%20Valid
      (bind _outactors (Actor|GetAllActorsOfClass "/Game/TwentyItems/Blueprints/ProceduralGeneration/ProceduralLevelManager.ProceduralLevelManager_C"))
      (bind _output_get (Variables|Territory|SetProceduralLevelManager (Utilities|Array|Get(acopy) _outactors)))))
  (return _output_get))

(fn FilterItemPickUpSpawnerLootables
  (params (Type :type InventoryItemType%20Enum :default "NewEnumerator0")))

(fn StartWaitingforPlayers
  (bind _output_get (References|GetDayNightCycleRef))
  ;[1 1 1] Sets Match State to Lobby
  (MatchState|SetMatchState)
  ;[1 1 1] Transitions from sunset to night time
  (Variables|/Game/TwentyItems/Blueprints/Main/BP_DayNightCycle.BP_DayNightCycle_C|SetTargetSunAngle _output_get 9e+01)
  (Variables|/Game/TwentyItems/Blueprints/Main/BP_DayNightCycle.BP_DayNightCycle_C|SetTargetTimeTransition _output_get 9e+01)
  ;[1 1 1] Starts counting down while waiting for players to start game
  (Variables|MatchState|SetLobbyTimeCountDown (Variables|MatchStateParameters|GetLobbyWaitTime))
  (bind _returnvalue (Utilities|Time|SetTimerbyFunctionName 0 "LobbyStartTimer" 1.0 true))
  (Variables|MatchState|SetLobbyStartTimerHandle _returnvalue))

(fn GetDayNightCycleRef
  (Utilities|IsValid (Variables|MatchState|GetBP_DayNightCycle)
    (:Is%20Valid
      _)
    (:Is%20Not%20Valid
      (bind _outactors (Actor|GetAllActorsOfClass "/Game/TwentyItems/Blueprints/Main/BP_DayNightCycle.BP_DayNightCycle_C"))
      (bind _output_get (Variables|MatchState|SetBP_DayNightCycle (Utilities|Array|Get(acopy) _outactors)))))
  (return _output_get))

(fn PreparetoStartGameFunction
  (bind _output_get (References|GetDayNightCycleRef))
  (bind _startmatchtime (Variables|MatchStateParameters|GetStartMatchTime))
  (MatchState|SetMatchState 1)
  ;[1 1 1] Transitions from sunset to night time
  (Variables|/Game/TwentyItems/Blueprints/Main/BP_DayNightCycle.BP_DayNightCycle_C|SetTargetSunAngle _output_get 9e+01)
  (Variables|/Game/TwentyItems/Blueprints/Main/BP_DayNightCycle.BP_DayNightCycle_C|SetTargetTimeTransition _output_get 1e+01)
  ;[1 1 1] Sets Time left to start match on the gamemode and replicated on the gamestate
  (Variables|MatchState|SetTimeLeftToStartMatch _startmatchtime)
  (Variables|/Game/TwentyItems/Blueprints/Main/GS_ExpressLaneOLD.GS_ExpressLaneOLD_C|SetTimeUntilGameStarts (References|GetGameStateReference) _startmatchtime)
  ;[1 1 1] Starts the countdown to begin the game
  (MatchState|StartGameTimer)
  (bind _returnvalue (Utilities|Time|SetTimerbyFunctionName 0 "StartGameTimer" 1.0 true))
  (Variables|MatchState|SetGameStartTimerHandle _returnvalue)
  ;[1 1 1] Spawns a bombay for each team
  (Bombay|SpawnBombays))

(fn StartGameFunction
  ;[1 1 1] Sets Players in the preparation phase
  (MatchState|SetMatchState 2)
  ;[1 1 1] Players can be damaged now that the game has started
  (Variables|GamePlayParameters|SetPlayersInvulnerable false)
  ;[1 1 1] Sets Match Started to True
  (Variables|MatchState|SetMatchStarted? true)
  ;[1 1 1] Prepares For Next Lights out Phase
  (MatchState|SetLightsOutTimer)
  ;[1 1 1] Spawns Players at their Bombay
  (Spawning|SpawnPlayersonMatchBegin))

(fn SetMatchState
  (params (MatchState%20 :type Integer))
  (Variables|MatchState|SetMatchState%20 MatchState%20)
  (Variables|/Game/TwentyItems/Blueprints/Main/GS_ExpressLaneOLD.GS_ExpressLaneOLD_C|SetMatchState%20 (References|GetGameStateReference) MatchState%20))

(fn LightsOutFunction
  (MatchState|SetMatchState 3)
  (Default|InitiateLightsOut (References|GetGameStateReference))
  (Variables|MatchState|SetLightsOut? true)
  (CallFunction|LightsonCountdown))

(fn LightsonCountDownFunction
  (bind _returnvalue (Utilities|Time|SetTimerbyFunctionName 0 "LightsOnTimerFunction" (Variables|MatchStateParameters|GetTimeUntilLightsComeUp)))
  (Variables|MatchState|SetLightsOnTimerHandle _returnvalue))

(fn LightsonTimerFunction
  (CallFunction|StartOvertimePhase))

(fn StartOverTimePhaseFunction
  (bind _output_get (References|GetDayNightCycleRef))
  (MatchState|SetMatchState 4)
  ;[1 1 1] Transitions from nighttime to dawn
  (Variables|/Game/TwentyItems/Blueprints/Main/BP_DayNightCycle.BP_DayNightCycle_C|SetTargetSunAngle _output_get 1.5e+02)
  (Variables|/Game/TwentyItems/Blueprints/Main/BP_DayNightCycle.BP_DayNightCycle_C|SetTargetTimeTransition _output_get (Variables|MatchStateParameters|GetOverTimePhaseLength))
  ;[1 1 1] Destroys all Bombays
  (Bombay|DestroyAllBombays)
  ;[1 1 1] Tells Players All Bombays Were Destroyed
  (Default|SendPlayersMessage (References|GetGameStateReference) "Dawn is Approaching 
All Bombays Were Destroyed!" "(R=1.000000,G=0.000000,B=0.000000,A=1.000000)"))

(fn DestroyAllBombays
  (Networking|SwitchHasAuthority
    (:Authority
      (Networking|SwitchHasAuthority
        (:Authority
          ;[1 1 1] Destroys all bombays that are still alive
          (for _array_element (Variables|/Game/TwentyItems/Blueprints/Main/GS_ExpressLaneOLD.GS_ExpressLaneOLD_C|GetTeams (References|GetGameStateReference))
            (if (not (Variables|/Game/TwentyItems/Blueprints/Main/Skylands/TeamActorOLD.TeamActorOLD_C|GetBombayDestroyed? _array_element))
              _)))))))

(fn HandlePlayerDeath
  (params (Player%20Controller :type Player%20Controller%20Object%20Reference) (Instigating%20Player%20State :type %20Object%20Reference))
  (LocalVariables|SetPlayerController Player%20Controller))

(fn IsTeamEliminated
  (params (Team :type Team%20Actor%20OLD%20Object%20Reference)))

(fn GetTeamsNotEliminated
  (bind _teamsleft (LocalVariables|GetTeamsLeft))
  ;[1 1 1] Adds every team that isn't eliminated
  (for _array_element (Variables|/Game/TwentyItems/Blueprints/Main/GS_ExpressLaneOLD.GS_ExpressLaneOLD_C|GetTeams (References|GetGameStateReference))
    (if (not false)
      (Utilities|Array|Add (LocalVariables|GetTeamsLeft) _array_element)))
  (return _teamsleft (Utilities|Array|Length _teamsleft)))

(fn EndGameFunction
  ;[1 1 1] Stops All Ongoing Timers for match states
  (MatchState|CancelAllMatchStates)
  ;[1 1 1] When the match ends players can't take damage anymore
  (Variables|GamePlayParameters|SetPlayersInvulnerable true)
  ;[1 1 1] Sets Match Ended To True
  (Variables|MatchState|SetMatchEnded? true)
  ;[1 1 1] Plays the victory effects from the gamestate
  (Default|PlayVictoryEffects (References|GetGameStateReference)))

(fn SpawnPlayerasSpectator
  (params (Player :type Player%20Controller%20Object%20Reference))
  ;[1 1 1] Spawns and possesses the expresslane spectator pawn
  (bind _returnvalue (Game|SpawnActorfromClass "/Game/TwentyItems/Blueprints/Player/ExpressLaneSpectatorPawn.ExpressLaneSpectatorPawn_C" (Math|Transform|MakeTransform "0, 0, 0" "0, 0, 0" "1,1,1") "AdjustIfPossibleButAlwaysSpawn" 0 0))
  (Pawn|Possess Player _returnvalue))

(fn CancelAllMatchStates
  (bind _gamestarttimerhandle (Variables|MatchState|GetGameStartTimerHandle))
  (bind _lobbystarttimerhandle (Variables|MatchState|GetLobbyStartTimerHandle))
  (bind _lightsontimerhandle (Variables|MatchState|GetLightsOnTimerHandle))
  (bind _lightsouttimerhandle (Variables|MatchState|GetLightsOutTimerHandle))
  (Utilities|FlowControl|Sequence
    (:then_0
      ;[1 1 1] Game Start Timer
      (if (Utilities|Time|IsValidTimerHandle _gamestarttimerhandle)
        (Utilities|Time|ClearandInvalidateTimerbyHandle _gamestarttimerhandle)))
    (:then_1
      ;[1 1 1] Lobby Start Timer
      (if (Utilities|Time|IsValidTimerHandle _lobbystarttimerhandle)
        (Utilities|Time|ClearandInvalidateTimerbyHandle _lobbystarttimerhandle)))
    (:then_2
      ;[1 1 1] Lights Out Timer Handle
      (if (Utilities|Time|IsValidTimerHandle _lightsouttimerhandle)
        (Utilities|Time|ClearandInvalidateTimerbyHandle _lightsouttimerhandle)))
    (:then_3
      ;[1 1 1] Lights On Timer Handle
      (if (Utilities|Time|IsValidTimerHandle _lightsontimerhandle)
        (Utilities|Time|ClearandInvalidateTimerbyHandle _lightsontimerhandle)))))