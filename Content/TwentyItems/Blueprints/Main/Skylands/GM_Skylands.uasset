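; GM_Skylands is the Skylands game mode, running a team match from lobby wait through a locked countdown to match start and a Bombay placement grace period.
; It spawns a ring of center-island pedestals and a force field, assigns pedestals randomly, and pins players there on Tick until start.
; Timers drive the phases and update GS_Skylands.
; Team assignment, Bombay handout, death handling and respawn are stubbed or disconnected.
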(event EventBeginPlay
  ;[1 0 0] Event Begin Play | places center island spawn points
  ;;[1 1 1] Makes sure no bloke is hacking
  (if (Networking|IsServer)
    ;;[1 1 1] Places Spawn Points where pedestals go in the center island
    (Spawning|CreateCenterIslandSpawnPoints)
    ;;[1 1 1] Spawns Players who were already loaded into the game
    (Spawning|SpawnLoadedPlayersatStart)
    ;;[1 1 1 1 14] Spawns Force Field barrier to block players from leaving the center island at the beginning of the match
    (MatchState|CreateForceFieldBarrier)
    ;;[1 1 1] Initiates the match state
    (CallFunction|StartWaitingforGametoStart)))

(event EventPostLogin
  (params (NewPlayer :type Player%20Controller%20Object%20Reference))
  ;[1 0 0] Log in and Log Out
  (Utilities|Array|Add (Variables|Players|GetPlayersInGame) NewPlayer)
  (Teams|HandleAddingPlayertoTeam NewPlayer)
  (Spawning|HandleSpawningNewPlayer NewPlayer))

(event EventOnLogout
  (params (ExitingController :type Controller%20Object%20Reference))
  (bind (_asplayer_controller _bsuccess) (Utilities|Casting|CastToPlayerController ExitingController))
  ;[1 0 0] Log in and Log Out
  (Utilities|Array|RemoveItem (Variables|Players|GetPlayersInGame) _asplayer_controller)
  (if (not _bsuccess)
    (Development|PrintString "PLAYER CONTROLLER POST LOGOUT FAILURE" true true "(R=1.000000,G=1.000000,B=0.000000,A=1.000000)" 4e+01)))

(event EventTick
  (params (DeltaSeconds :type Float%20%28single-precision%29))
  ;[1 1 1] Event Tick
  (Players|HandlePlayerLocksonTick))

(event Custom|StartWaitingForGameToStart
  ;[1 0 0] Start Waiting For Game To Start | Sets lobby wait Timer
  (bind _returnvalue (Utilities|Time|SetTimerbyEvent (delegate Custom|PrepareToStartMatch) (Variables|MatchStateParameters|GetLobbyWaitTime)))
  (Variables|MatchStateTimers|SetWaitingForGameToStartTimer _returnvalue))

(event Custom|PrepareToStartMatch
  ;[1 0 0] Prepare to Start Match | Sets timer countdown for the game to start and respawns all players at prdestals with locked movement
  (Utilities|Time|ClearandInvalidateTimerbyHandle (Variables|MatchStateTimers|GetWaitingForGameToStartTimer))
  ;;[1 1 1] Respawns players at pedestals and locks their movement there until the game starts
  (Spawning|ResetPlayersatPedestal)
  ;;[1 1 1] Sets time to countdown and relays to game state for replication
  (MatchState|SetUpPreparetoStartGameTimer)
  ;;[1 1 1] Sets Timer to loop until 0 is reached and game starts
  (bind _returnvalue (Utilities|Time|SetTimerbyFunctionName 0 "PrepareToStartGameTimerFunction" 1.0 true))
  (Variables|MatchStateTimers|SetPrepareToStartGameTimer _returnvalue))

(event Custom|StartMatch
  ;[1 0 0] Start Match
  (Utilities|Time|ClearandInvalidateTimerbyHandle (Variables|MatchStateTimers|GetPrepareToStartGameTimer))
  ;;[1 1 1] Sets timer to build base and place bombays
  (bind _returnvalue (Utilities|Time|SetTimerbyEvent (delegate Custom|EndPreparationGracePeriod) (Variables|MatchStateParameters|GetPreparationGracePeriod)))
  (Variables|MatchStateTimers|SetPreparationGracePeriodTimer _returnvalue)
  ;;[1 1 1] Gives players back control of their characters
  (Players|UnlockAllPlayersfromLocation)
  ;;[1 1 1] Destroys center island barrier so players can leave the island
  (Actor|DestroyActor (Variables|MatchStateParameters|GetCenterIslandForceFieldBarrierRef))
  ;;[1 1 1] Gives every player a Bombay to Place
  (MatchState|GivePlayersBombays)
  ;;[1 1 1] Sets the match to started on the game state and players become vulnerable
  (Variables|/Game/TwentyItems/Blueprints/Main/Skylands/GS_Skylands.GS_Skylands_C|SetMatchStarted? (References|GetGameStateRef) true)
  (Variables|MatchStateTimers|SetPlayersInvulnerable? false)
  ;;[1 1 1] Tells players to place their bombay
  (Utilities|FlowControl|Delay 2.0)
  (Default|SendGameStateNotification (References|GetGameStateRef) "Place Your Bombay in The Name Of Tcalvin" 5.0))

(event Custom|EndPreparationGracePeriod
  ;[1 0 0] End Preparation Grace Period; Bombays are no longer invulnerable and the buffoonery has officially begun
  ;;[1 1 1] Clears Grace period timer
  (Utilities|Time|ClearandInvalidateTimerbyHandle (Variables|MatchStateTimers|GetPreparationGracePeriodTimer))
  ;;[1 1 1] Sets Grace Period Ended; Bombays are no longer invulnerable
  (Variables|/Game/TwentyItems/Blueprints/Main/Skylands/GS_Skylands.GS_Skylands_C|SetPreparationGracePeriodEnded? (References|GetGameStateRef) true)
  (Variables|MatchStateTimers|SetBombaysInvulnerable? false)
  ;;[1 1 1] Notifies Players that the grace period has ended
  (Default|SendGameStateNotification (References|GetGameStateRef) "The Grace Period Has Ended 
Bombays Are No Longer Invulnerable" 5.0)
  ;;[1 1 1 1 12] If a team didn't place their bombay by the time the grace period has ended, their bombay is set as destroyed
  (Teams|HandleBombaysThatWereNotPlaced))

(fn ConstructionScript)

(fn CreateCenterIslandSpawnPoints
  (if (Networking|IsServer)
    ;[0 0 0] Given the radius that the pedestals will spawn across and the height the player starts will be, the spawn points are spawned around a cricle
    (for _index (range 0 (- (Variables|Players|GetMaxPlayers) 1))
      (bind _returnvalue (Game|SpawnActorfromClass "/Game/TwentyItems/Blueprints/Main/Skylands/CenterIslandSpawnPoint.CenterIslandSpawnPoint_C" (Math|Transform|MakeTransform (Math|Vector|MakeVector (.X (Math|Vector2D|BreakVector2D (.Location (CallFunction|PlaceItemAlongCircle _index (Variables|Players|GetMaxPlayers) (Variables|Spawning|GetCenterIslandSpawnRadius))))) (.Y (Math|Vector2D|BreakVector2D (.Location (CallFunction|PlaceItemAlongCircle _index (Variables|Players|GetMaxPlayers) (Variables|Spawning|GetCenterIslandSpawnRadius))))) (Variables|Spawning|GetSpawnPointHeight)) (Math|Rotator|MakeRotator 0.0 0.0 (+ (* _index (.DegreeIncrement (CallFunction|PlaceItemAlongCircle _index (Variables|Players|GetMaxPlayers) (Variables|Spawning|GetCenterIslandSpawnRadius)))) 1.8e+02)) "1,1,1") "AlwaysSpawn" 0 0))
      (Utilities|Array|Add (Variables|Spawning|GetCenterIslandSpawnPoints) _returnvalue))
    ;[1 1 1] Comment
    (Variables|Spawning|SetUnownedCenterIslandSpawnPoints (Variables|Spawning|GetCenterIslandSpawnPoints))))

(fn SpawnLoadedPlayersatStart
  (if (not (Variables|Spawning|GetSpawnedLoadedPlayersAtTheStart?))
    (Variables|Spawning|SetSpawnedLoadedPlayersAtTheStart? true)
    (for _array_element (Variables|Players|GetPlayersInGame)
      (Spawning|SpawnCharacteronPedestal _array_element))))

(fn HandleSpawningNewPlayer
  (params (New%20Player :type Player%20Controller%20Object%20Reference))
  (Spawning|SpawnPlayeratPedestal New%20Player))

(fn SpawnPlayeratPedestal
  (params (Player :type Player%20Controller%20Object%20Reference))
  (if (Variables|Spawning|GetSpawnedLoadedPlayersAtTheStart?)
    (Spawning|SpawnCharacteronPedestal Player)))

(fn DoesPlayerOwnPedestal
  (params (Player :type Player%20Controller%20Object%20Reference))
  (LocalVariables|SetPlayerRef Player)
  (LocalVariables|SetFoundSpawnPoint false)
  (bind (_array_element _array_index) (Utilities|Array|ForEachLoopwithBreak (Variables|Spawning|GetCenterIslandSpawnPoints) :!label _label)
    (:LoopBody
      (if (== (Variables|/Game/TwentyItems/Blueprints/Main/Skylands/CenterIslandSpawnPoint.CenterIslandSpawnPoint_C|GetOwningPlayer _array_element) (LocalVariables|GetPlayerRef))
        (LocalVariables|SetFoundSpawnPoint true)
        (LocalVariables|SetIndex _array_index)
        (goto _label Break)))
    (:Completed
      (return (LocalVariables|GetFoundSpawnPoint) (LocalVariables|GetIndex)))))

(fn AssignPlayerPedestal
  (params (Player :type Player%20Controller%20Object%20Reference))
  (bind _unownedcenterislandspawnpoints (Variables|Spawning|GetUnownedCenterIslandSpawnPoints))
  (LocalVariables|SetPlayer%20Ref Player)
  (Utilities|FlowControl|Sequence
    (:then_0
      ;[1 1 1] Adds all the spawn pedestal indexes to an array to be selected from
      (bind _output_get (LocalVariables|SetSelectedIndex (Math|Random|RandomIntegerinRange 0 (Utilities|Array|LastIndex _unownedcenterislandspawnpoints))))
      (Variables|/Game/TwentyItems/Blueprints/Main/Skylands/CenterIslandSpawnPoint.CenterIslandSpawnPoint_C|SetOwningPlayer (Utilities|Array|Get(acopy) _unownedcenterislandspawnpoints _output_get) (LocalVariables|GetPlayer%20Ref))
      (LocalVariables|SetIndex (Utilities|Array|Get(acopy) _unownedcenterislandspawnpoints _output_get))
      (Utilities|Array|RemoveIndex (Variables|Spawning|GetUnownedCenterIslandSpawnPoints) _output_get))
    (:then_1
      (return (LocalVariables|GetIndex)))))

(fn SpawnCharacteronPedestal
  (params (Player%20Controller :type Player%20Controller%20Object%20Reference))
  (bind _output_get (LocalVariables|SetPlayerRef Player%20Controller))
  (bind _spawn_pedestal (Spawning|AssignPlayerPedestalifUnowned _output_get))
  (bind _returnvalue (Game|SpawnActorfromClass "/Game/TwentyItems/Blueprints/Player/ExpressLaneCharacter.ExpressLaneCharacter_C" (Math|Transform|MakeTransform (.location (Transformation|GetWorldTransform (Variables|/Game/TwentyItems/Blueprints/Main/Skylands/CenterIslandSpawnPoint.CenterIslandSpawnPoint_C|GetArrow _spawn_pedestal))) (.rotation (Transformation|GetWorldTransform (Variables|/Game/TwentyItems/Blueprints/Main/Skylands/CenterIslandSpawnPoint.CenterIslandSpawnPoint_C|GetArrow _spawn_pedestal))) "1,1,1") "AdjustIfPossibleButAlwaysSpawn" _output_get (.rotation (Transformation|GetWorldTransform (Variables|/Game/TwentyItems/Blueprints/Main/Skylands/CenterIslandSpawnPoint.CenterIslandSpawnPoint_C|GetArrow _spawn_pedestal))) 0 0))
  (Pawn|Possess (LocalVariables|GetPlayerRef) _returnvalue)
  (return _returnvalue))

(fn AssignPlayerPedestalifUnowned
  (params (Player :type Player%20Controller%20Object%20Reference))
  (bind (_owns_pedestal_ _pedestal_index) (Spawning|DoesPlayerOwnPedestal Player))
  (LocalVariables|SetPlayer%20Ref Player)
  (Utilities|FlowControl|Sequence
    (:then_0
      (if _owns_pedestal_
        (LocalVariables|SetSpawnPedestal (Utilities|Array|Get(acopy) (Variables|Spawning|GetCenterIslandSpawnPoints) _pedestal_index))
        (else
          (bind _assigned_pedestal (Spawning|AssignPlayerPedestal (LocalVariables|GetPlayer%20Ref)))
          (LocalVariables|SetSpawnPedestal _assigned_pedestal))))
    (:then_1
      (return (LocalVariables|GetSpawnPedestal)))))

(fn ResetPlayersatPedestal
  (Spawning|DestroyAllCharacters)
  (for _array_element (Variables|Players|GetPlayersInGame)
    (bind _spawnedcharacter (Spawning|SpawnCharacteronPedestal _array_element))
    (Default|DisableActions _spawnedcharacter false false false false true true false false false false false false false false false false false false true false false)
    (Players|LockPlayerinLocation _spawnedcharacter)))

(fn DestroyAllCharacters
  (for _array_element (Variables|Players|GetPlayersInGame)
    (if (CallFunction|ClassEqual? (Pawn|GetControlledPawn _array_element) "/Game/TwentyItems/Blueprints/Player/ExpressLaneCharacter.ExpressLaneCharacter_C")
      (Default|CommitDrinkBleachFunction (.AsExpress%20Lane%20Character (Utilities|Casting|CastToExpressLaneCharacter (Pawn|GetControlledPawn _array_element))) 0 0 true))))

(fn LockPlayerinLocation
  (params (Player :type Express%20Lane%20Character%20Object%20Reference))
  (bind _lockedplayersinlocation (Variables|Players|GetLockedPlayersInLocation))
  (Utilities|FlowControl|Sequence
    (:then_0
      (if (Utilities|Map|Contains _lockedplayersinlocation Player)
        (Utilities|Map|Remove (Variables|Players|GetLockedPlayersInLocation) Player)))
    (:then_1
      (Utilities|Map|Add _lockedplayersinlocation Player (Transformation|GetActorLocation Player)))))

(fn HandlePlayerLocksonTick
  (bind _lockedplayersinlocation (Variables|Players|GetLockedPlayersInLocation))
  (if (> (Utilities|Map|Length _lockedplayersinlocation) 0)
    (bind _keys (Utilities|Map|Keys _lockedplayersinlocation))
    (for _array_element _keys
      (if (.ReturnValue (Utilities|Map|Find _lockedplayersinlocation _array_element))
        (Transformation|SetActorLocation _array_element (.Value (Utilities|Map|Find _lockedplayersinlocation _array_element)) false true)))))

(fn PreparetoStartGameTimerFunction
  (bind _result (Math|Integer|DecrementInt (Variables|MatchStateTimers|GetTimeLeftUntilGameStarts))
    (:%20%20
      (Variables|/Game/TwentyItems/Blueprints/Main/Skylands/GS_Skylands.GS_Skylands_C|SetTimeUntilGameStarts (References|GetGameStateRef) _result)
      (if (<= (Variables|MatchStateTimers|GetTimeLeftUntilGameStarts) 0)
        (CallFunction|StartMatch)))))

(fn GetGameStateRef
  (Utilities|IsValid (Variables|References|GetGS%20Skylands)
    (:Is%20Valid
      _)
    (:Is%20Not%20Valid
      (Variables|References|SetGS%20Skylands (.AsGS%20Skylands (Utilities|Casting|CastToGS_Skylands (Game|GetGameState))))))
  (return (Variables|References|GetGS%20Skylands)))

(fn SetUpPreparetoStartGameTimer
  (bind _output_get (Variables|MatchStateTimers|SetTimeLeftUntilGameStarts (Math|Float|Truncate (Variables|MatchStateParameters|GetPrepareToStartGameTime))))
  (Variables|/Game/TwentyItems/Blueprints/Main/Skylands/GS_Skylands.GS_Skylands_C|SetTimeUntilGameStarts (References|GetGameStateRef) _output_get))

(fn UnlockAllPlayersfromLocation
  (bind _lockedplayersinlocation (Variables|Players|GetLockedPlayersInLocation))
  (Utilities|FlowControl|Sequence
    (:then_0
      (bind _keys (Utilities|Map|Keys _lockedplayersinlocation))
      (for _array_element _keys
        (Default|DisableActions _array_element false false false false true true false false false false false false false false false false false false true false true)))
    (:then_1
      (Utilities|Map|Clear _lockedplayersinlocation))))

(fn GetProceduralSkylandsManagerRef
  (Utilities|IsValid (Variables|References|GetProceduralSkylandManager)
    (:Is%20Valid
      _)
    (:Is%20Not%20Valid
      (bind _outactors (Actor|GetAllActorsOfClass "/Game/TwentyItems/Blueprints/ProceduralGeneration/Skylands/Main/ProceduralSkylandManager.ProceduralSkylandManager_C"))
      (bind _output_get (Variables|References|SetProceduralSkylandManager (Utilities|Array|Get(acopy) _outactors)))))
  (return _output_get))

(fn CreateForceFieldBarrier
  ;[1 1 1] Spawns Force Field Barrier for the beginning of the match
  (bind _returnvalue (Game|SpawnActorfromClass "/Game/TwentyItems/Blueprints/Main/Skylands/ForceFieldBarrier.ForceFieldBarrier_C" (Math|Transform|MakeTransform "0, 0, 0" "0, 0, 0" "1,1,1") "Undefined" 0 (Variables|/Game/TwentyItems/Blueprints/ProceduralGeneration/Skylands/Main/ProceduralSkylandManager.ProceduralSkylandManager_C|GetMainIslandRadius (References|GetProceduralSkylandsManagerRef)) 0))
  (Variables|MatchStateParameters|SetCenterIslandForceFieldBarrierRef _returnvalue))

(fn HandleAddingPlayertoTeam
  (params (New%20Player :type Player%20Controller%20Object%20Reference))
  (LocalVariables|SetPlayerRef New%20Player))

(fn CreateTeam
  (bind _returnvalue (Game|SpawnActorfromClass "/Game/TwentyItems/Blueprints/Main/Skylands/TeamManager.TeamManager_C" (Math|Transform|MakeTransform "0, 0, 0" "0, 0, 0" "1,1,1") "AlwaysSpawn" 0 self "" 0))
  (Utilities|Array|Add (Variables|Teams|GetTeams) _returnvalue)
  (Utilities|Array|Add (Variables|/Game/TwentyItems/Blueprints/Main/Skylands/GS_Skylands.GS_Skylands_C|GetTeams (References|GetGameStateRef)) _returnvalue)
  (return _returnvalue))

(fn FindEmptyTeam
  (LocalVariables|SetTeam 0)
  (bind _array_element (Utilities|Array|ForEachLoopwithBreak (Variables|Teams|GetTeams) :!label _label)
    (:LoopBody
      (if (Default|DoesTeamHaveSpace _array_element)
        (LocalVariables|SetTeam _array_element)
        (goto _label Break)))
    (:Completed
      (return (Utilities|IsValid (LocalVariables|GetTeam)) (LocalVariables|GetTeam)))))

(fn HandlePlayerDeath
  (params (Player%20Controller :type %20Object%20Reference) (Killed%20Player :type %20Object%20Reference) (Instigator :type %20Object%20Reference))
  (LocalVariables|SetController%20Ref 0)
  (LocalVariables|SetInstigatorRef 0)
  (LocalVariables|SetKilled%20Player%20Ref 0)
  (Utilities|FlowControl|Sequence
    (:then_1
      (return (LocalVariables|GetElimination?)))))

(fn OnSeedGenerated)

(fn InstructFloorLootSpawns
  (bind _floorlootspawnrange (Variables|LootParameters|GetFloorLootSpawnRange))
  ;[1 1 1] Gets all floor loot spawners
  (bind _outactors (Actor|GetAllActorsOfClass "/Game/TwentyItems/Blueprints/Lootables/Skylands/FloorLoot_Parent.FloorLoot_Parent_C"))
  (Variables|Loot|SetFloorLootSpawners _outactors)
  (Utilities|FlowControl|Sequence
    (:then_0
      ;[1 1 1] Determines how much floor loot should be spawned
      (LocalVariables|SetFloorLootSpawns (Math|Random|RandomIntegerinRangefromStream (.x _floorlootspawnrange) (.y _floorlootspawnrange) (Variables|/Game/TwentyItems/Blueprints/ProceduralGeneration/Skylands/Main/ProceduralSkylandManager.ProceduralSkylandManager_C|GetRandomSeed (References|GetProceduralSkylandsManagerRef)))))
    (:then_1
      ;[1 1 1] Keeps Adding Spawners Until the amount of loot spawners selected matches the desired amount or until all are selected
      (while (and (!= (Utilities|Array|Length (LocalVariables|GetSelectedLootSpawners)) (LocalVariables|GetFloorLootSpawns)) (> (Utilities|Array|Length (Variables|Loot|GetFloorLootSpawners)) 0))
        ;[1 1 1] Gets Random Selections until the quota of floor loot spawns is filled
        (bind _output_get (LocalVariables|SetCurrentIndex (Math|Random|RandomIntegerinRangefromStream 0 (Utilities|Array|LastIndex (Variables|Loot|GetFloorLootSpawners)) (Variables|/Game/TwentyItems/Blueprints/ProceduralGeneration/Skylands/Main/ProceduralSkylandManager.ProceduralSkylandManager_C|GetRandomSeed (References|GetProceduralSkylandsManagerRef)))))
        (Utilities|Array|AddUnique (LocalVariables|GetSelectedLootSpawners) (Utilities|Array|Get(acopy) (Variables|Loot|GetFloorLootSpawners) _output_get))
        (Utilities|Array|RemoveIndex (Variables|Loot|GetFloorLootSpawners) _output_get)))
    (:then_2
      ;[1 1 1] Instructs selected floor loot spawners and removes the rest
      (for _array_element (Variables|Loot|GetFloorLootSpawners)
        (Actor|DestroyActor _array_element))
      (for _array_element_2 (LocalVariables|GetSelectedLootSpawners)
        (Default|ReceivedSeed _array_element_2)))))

(fn RespawnPlayeratBombay
  (params (Player :type %20Object%20Reference)))

(fn SpawnLootPortals)

(fn AttemptEliminateTeam
  (params (Team :type Team%20Manager%20Object%20Reference))
  (LocalVariables|SetTeam%20Ref Team)
  (Utilities|FlowControl|Sequence
    (:then_0
      ;[1 1 1] Makes sure the grace period has ended
      (if (Variables|/Game/TwentyItems/Blueprints/Main/Skylands/GS_Skylands.GS_Skylands_C|GetPreparationGracePeriodEnded? (References|GetGameStateRef))
        ;[1 1 1] Checks if the team has a bombay
        (if (or (Variables|/Game/TwentyItems/Blueprints/Main/Skylands/TeamManager.TeamManager_C|GetBombayDestroyed? (LocalVariables|GetTeam%20Ref)) (not (Variables|/Game/TwentyItems/Blueprints/Main/Skylands/TeamManager.TeamManager_C|GetHasBombayBeenPlaced? (LocalVariables|GetTeam%20Ref))))
          ;[1 1 1] Checks if every member in the team is eliminated
          (if (Default|AreAllMembersEliminated (LocalVariables|GetTeam%20Ref))
            ;[1 1 1] Eliminates Team
            (Variables|/Game/TwentyItems/Blueprints/Main/Skylands/TeamManager.TeamManager_C|SetTeamEliminated? (LocalVariables|GetTeam%20Ref) true)
            (LocalVariables|SetEliminatedTeam? true)))))
    (:then_1
      (return (LocalVariables|GetEliminatedTeam?)))))

(fn HandleBombaysThatWereNotPlaced
  (for _array_element (Variables|Teams|GetTeams)
    (if (not (Variables|/Game/TwentyItems/Blueprints/Main/Skylands/TeamManager.TeamManager_C|GetHasBombayBeenPlaced? _array_element))
      (Variables|/Game/TwentyItems/Blueprints/Main/Skylands/TeamManager.TeamManager_C|SetBombayDestroyed? _array_element true))))

(fn IsOneTeamStanding?
  (bind _array_element (Utilities|Array|ForEachLoopwithBreak (Variables|Teams|GetTeams) :!label _label)
    (:LoopBody
      (if (not (Variables|/Game/TwentyItems/Blueprints/Main/Skylands/TeamManager.TeamManager_C|GetTeamEliminated? _array_element))
        (Utilities|IsValid (LocalVariables|GetWinningTeam)
          (:Is%20Valid
            (LocalVariables|SetIsGameOver? false)
            (goto _label Break))
          (:Is%20Not%20Valid
            (LocalVariables|SetWinningTeam _array_element)
            (LocalVariables|SetIsGameOver? true)))))
    (:Completed
      (return (LocalVariables|GetIsGameOver?) (LocalVariables|GetWinningTeam)))))

(fn EndMatch
  (params (Winning%20Team :type Team%20Manager%20Object%20Reference))
  (LocalVariables|SetWinningTeam Winning%20Team)
  ;[1 1 1] Players Can no longer take damage once the game has ended
  (Variables|MatchStateTimers|SetPlayersInvulnerable? true)
  ;[1 1 1] Plays Victory Effects on GameState
  (Default|PlayVictoryEffects (References|GetGameStateRef)))

(fn GivePlayersBombays
  (for _array_element (Variables|/Game/TwentyItems/Blueprints/Main/Skylands/GS_Skylands.GS_Skylands_C|GetTeams (References|GetGameStateRef))
    _))