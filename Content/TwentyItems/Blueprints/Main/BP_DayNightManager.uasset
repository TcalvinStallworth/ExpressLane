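; Day/night manager that changes the level's atmosphere based on which day/night box the player is in.
; On BeginPlay it caches the first sky sphere, directional light, height fog and skylight found.
; Each tick it targets the first in-range box, else DefaultBox, and uses that box's transition alpha to blend from DefaultBox settings.
; The blend drives sun angle (offset by box rotation), light intensities, skylight cubemaps, fog, clouds and stars.
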(event EventBeginPlay
  (References|GetSkyReferences))

(event Collision|EventActorBeginOverlap
  (params (OtherActor :type Actor%20Object%20Reference)))

(event EventTick
  (params (DeltaSeconds :type Float%20%28single-precision%29))
  (Utilities|FlowControl|Sequence
    (:then_0
      (bind (_found_target_ _indexeth) (CallFunction|FindActiveDayNightBox))
      (if _found_target_
        (Variables|Default|SetCurrentDayNightBoxTarget (Utilities|Array|Get(acopy) (Variables|Default|GetDayNightBoxes) _indexeth))
        (else
          (Variables|Default|SetCurrentDayNightBoxTarget (Variables|Default|GetDefaultBox)))))
    (:then_1
      (Utilities|IsValid (Variables|Default|GetDefaultBox)
        (:Is%20Valid
          (bind _alpha (Default|GetTransitionAlpha (Variables|Default|GetCurrentDayNightBoxTarget)))
          (CallFunction|UpdateAtmosphere _alpha))))))

(fn ConstructionScript)

(fn FindActiveDayNightBox
  (LocalVariables|SetFoundBox false)
  (bind (_array_element _array_index) (Utilities|Array|ForEachLoopwithBreak (Variables|Default|GetDayNightBoxes) :!label _label)
    (:LoopBody
      (if (Default|PlayerinRange? _array_element)
        (LocalVariables|SetIndex _array_index)
        (LocalVariables|SetFoundBox true)
        (goto _label Break)))
    (:Completed
      (return (LocalVariables|GetFoundBox) (LocalVariables|GetIndex)))))

(fn UpdateAtmosphere
  (params (Alpha :type Float%20%28single-precision%29))
  (LocalVariables|SetAlphae Alpha)
  (Sun|UpdateSun (LocalVariables|GetAlphae))
  (SkyLight|UpdateSkyLight (LocalVariables|GetAlphae))
  (Fog|UpdateExponentialHeightFog (LocalVariables|GetAlphae))
  (Sky|UpdateSky (LocalVariables|GetAlphae)))

(fn GetSkyReferences
  (Utilities|FlowControl|Sequence
    (:then_0
      (bind _outactors (Actor|GetAllActorsOfClass "/Engine/EngineSky/BP_Sky_Sphere.BP_Sky_Sphere_C"))
      (Variables|References|SetSkyDome (Utilities|Array|Get(acopy) _outactors)))
    (:then_1
      (bind _outactors_2 (Actor|GetAllActorsOfClass "/Script/Engine.DirectionalLight"))
      (Variables|References|SetSun (Utilities|Array|Get(acopy) _outactors_2)))
    (:then_2
      (bind _outactors_3 (Actor|GetAllActorsOfClass "/Script/Engine.ExponentialHeightFog"))
      (Variables|References|SetExponentialHeightFogRef (Utilities|Array|Get(acopy) _outactors_3)))
    (:then_3
      (bind _outactors_4 (Actor|GetAllActorsOfClass "/Script/Engine.SkyLight"))
      (Variables|References|SetSkyLightRef (Utilities|Array|Get(acopy) _outactors_4)))))

(fn GetGameStateRef
  (Utilities|IsValid (Variables|References|GetGS%20Skylands)
    (:Is%20Valid
      _)
    (:Is%20Not%20Valid
      (bind _output_get (Variables|References|SetGS%20Skylands (.AsGS%20Skylands (Utilities|Casting|CastToGS_Skylands (Game|GetGameState)))))))
  (return _output_get))

(fn UpdateSun
  (params (Alpha :type Float%20%28single-precision%29))
  (bind _sun (Variables|References|GetSun))
  (bind _skydome (Variables|References|GetSkyDome))
  (bind _currentdaynightboxtarget (Variables|Default|GetCurrentDayNightBoxTarget))
  (Utilities|IsValid _sun
    (:Is%20Valid
      (Transformation|SetActorRotation _sun (Math|Rotator|Lerp(Rotator) (Variables|/Game/TwentyItems/Blueprints/Main/BP_DayNightBox.BP_DayNightBox_C|GetTargetSunAngle (Variables|Default|GetDefaultBox)) (Math|Rotator|CombineRotators (Variables|/Game/TwentyItems/Blueprints/Main/BP_DayNightBox.BP_DayNightBox_C|GetTargetSunAngle _currentdaynightboxtarget) (Transformation|GetActorRotation _currentdaynightboxtarget)) Alpha true))
      (Rendering|Components|Light|SetIntensity (Variables|/Script/Engine.Light|GetLightComponent (Variables|References|GetSun)) (Math|Float|Lerp (Variables|/Game/TwentyItems/Blueprints/Main/BP_DayNightBox.BP_DayNightBox_C|GetTargetSunIntensity (Variables|Default|GetDefaultBox)) (Variables|/Game/TwentyItems/Blueprints/Main/BP_DayNightBox.BP_DayNightBox_C|GetTargetSunIntensity (Variables|Default|GetCurrentDayNightBoxTarget)) Alpha))
      (Utilities|IsValid _skydome
        (:Is%20Valid
          (Default|UpdateSunDirection _skydome))))))

(fn UpdateSkyLight
  (params (Alpha :type Float%20%28single-precision%29))
  (bind _skylightref (Variables|References|GetSkyLightRef))
  (bind _lightcomponent (Variables|/Script/Engine.SkyLight|GetLightComponent _skylightref))
  (Utilities|IsValid _skylightref
    (:Is%20Valid
      (Rendering|Components|Light|SetIntensity _lightcomponent (Math|Float|Lerp (Variables|/Game/TwentyItems/Blueprints/Main/BP_DayNightBox.BP_DayNightBox_C|GetTargetSkyLightIntensity (Variables|Default|GetDefaultBox)) (Variables|/Game/TwentyItems/Blueprints/Main/BP_DayNightBox.BP_DayNightBox_C|GetTargetSkyLightIntensity (Variables|Default|GetCurrentDayNightBoxTarget)) Alpha))
      (Class|SkyLightComponent|SetCubemapBlend _lightcomponent (Variables|/Game/TwentyItems/Blueprints/Main/BP_DayNightBox.BP_DayNightBox_C|GetSkyLightCubeMap (Variables|Default|GetDefaultBox)) (Variables|/Game/TwentyItems/Blueprints/Main/BP_DayNightBox.BP_DayNightBox_C|GetSkyLightCubeMap (Variables|Default|GetCurrentDayNightBoxTarget)) Alpha))))

(fn UpdateExponentialHeightFog
  (params (Alpha :type Float%20%28single-precision%29))
  (bind _exponentialheightfogref (Variables|References|GetExponentialHeightFogRef))
  (bind _defaultbox (Variables|Default|GetDefaultBox))
  (bind _currentdaynightboxtarget (Variables|Default|GetCurrentDayNightBoxTarget))
  (bind _component (Variables|/Script/Engine.ExponentialHeightFog|GetComponent _exponentialheightfogref))
  (bind _fogdata (Variables|/Game/TwentyItems/Blueprints/Main/BP_DayNightBox.BP_DayNightBox_C|GetFogData _defaultbox))
  (bind _fogdata_2 (Variables|/Game/TwentyItems/Blueprints/Main/BP_DayNightBox.BP_DayNightBox_C|GetFogData _currentdaynightboxtarget))
  (bind (_fogdensity _foginscatteringcolor _fogheightfalloff _fogmaxopacity _startdistance _fogcutoffdistance _volumetricfog _scatteringdistribution _extinctionscale _viewdistance) (Utilities|Struct|BreakFogStruct _fogdata_2))
  (bind (_fogdensity_2 _foginscatteringcolor_2 _fogheightfalloff_2 _fogmaxopacity_2 _startdistance_2 _fogcutoffdistance_2 _volumetricfog_2 _scatteringdistribution_2 _extinctionscale_2 _viewdistance_2) (Utilities|Struct|BreakFogStruct _fogdata))
  (Utilities|IsValid _exponentialheightfogref
    (:Is%20Valid
      (Class|ExponentialHeightFogComponent|SetFogDensity _component (Math|Float|Lerp _fogdensity_2 _fogdensity Alpha))
      (Class|ExponentialHeightFogComponent|SetFogInscatteringColor _component (Math|Color|Lerp(LinearColor) _foginscatteringcolor_2 _foginscatteringcolor Alpha))
      (Class|ExponentialHeightFogComponent|SetFogHeightFalloff _component (Math|Float|Lerp _fogheightfalloff_2 _fogheightfalloff Alpha))
      (Class|ExponentialHeightFogComponent|SetFogMaxOpacity _component (Math|Float|Lerp _fogmaxopacity_2 _fogmaxopacity Alpha))
      (Class|ExponentialHeightFogComponent|SetStartDistance _component (Math|Float|Lerp _startdistance_2 _startdistance Alpha))
      (Class|ExponentialHeightFogComponent|SetFogCutoffDistance _component (Math|Float|Lerp _fogcutoffdistance_2 _fogcutoffdistance Alpha))
      (Class|ExponentialHeightFogComponent|SetVolumetricFog _component (select (>= Alpha 0.5) _volumetricfog _volumetricfog_2))
      (Class|ExponentialHeightFogComponent|SetVolumetricFogScatteringDistribution _component (Math|Float|Lerp _scatteringdistribution_2 _scatteringdistribution Alpha))
      (Class|ExponentialHeightFogComponent|SetVolumetricFogExtinctionScale _component (Math|Float|Lerp _extinctionscale_2 _extinctionscale Alpha))
      (Class|ExponentialHeightFogComponent|SetVolumetricFogDistance _component (Math|Float|Lerp _viewdistance_2 _viewdistance Alpha)))))

(fn UpdateSky
  (params (Alpha :type Float%20%28single-precision%29))
  (bind _currentdaynightboxtarget (Variables|Default|GetCurrentDayNightBoxTarget))
  (bind _skydome (Variables|References|GetSkyDome))
  (bind _defaultbox (Variables|Default|GetDefaultBox))
  (Variables|/Engine/EngineSky/BP_Sky_Sphere.BP_Sky_Sphere_C|SetCloud%20opacity _skydome (Math|Float|Lerp (Variables|/Game/TwentyItems/Blueprints/Main/BP_DayNightBox.BP_DayNightBox_C|GetTargetCloudOpacity _defaultbox) (Variables|/Game/TwentyItems/Blueprints/Main/BP_DayNightBox.BP_DayNightBox_C|GetTargetCloudOpacity _currentdaynightboxtarget) Alpha))
  (Variables|/Engine/EngineSky/BP_Sky_Sphere.BP_Sky_Sphere_C|SetCloud%20speed _skydome (Math|Float|Lerp (Variables|/Game/TwentyItems/Blueprints/Main/BP_DayNightBox.BP_DayNightBox_C|GetTargetCloudSpeed _defaultbox) (Variables|/Game/TwentyItems/Blueprints/Main/BP_DayNightBox.BP_DayNightBox_C|GetTargetCloudSpeed _currentdaynightboxtarget) Alpha))
  (Variables|/Engine/EngineSky/BP_Sky_Sphere.BP_Sky_Sphere_C|SetStars%20brightness _skydome (Math|Float|Lerp (Variables|/Game/TwentyItems/Blueprints/Main/BP_DayNightBox.BP_DayNightBox_C|GetTargetStarBrightness _defaultbox) (Variables|/Game/TwentyItems/Blueprints/Main/BP_DayNightBox.BP_DayNightBox_C|GetTargetStarBrightness _currentdaynightboxtarget) Alpha))
  (Default|RefreshMaterial (Variables|References|GetSkyDome)))