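; Game State for the Express Lane game, apparently an older version, that drives match-wide presentation: team messages, preparation phase, lights-out and victory.
; MatchState's OnRep opens the preparation widget or calls an empty countdown stub.
; Lights-out plays a sound and fades the skylight on a timeline; the authority then sets TurnedLightsOff, whose OnRep applies dimmed lighting for clients that missed the multicast.
; Team assignment is unwired.
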(event Custom|SendPlayersMessage
  (params (Text%20 :type Text) (TextColor :type Linear%20Color%20Structure))
  ;[0.5 0 1] Send Players Message
  (bind _returnvalue (UserInterface|CreateWidget "/Game/TwentyItems/Blueprints/Player/UI/GameState/GameMode/W_TeamMessage.W_TeamMessage_C" 0 Text%20 TextColor))
  (UserInterface|Viewport|AddtoViewport _returnvalue 0))

(event EventBeginPlay)

(event EventTick
  (params (DeltaSeconds :type Float%20%28single-precision%29)))

(event Custom|InitiateLightsOut
  ;[1 0 0] Lights Out Event
  ;;[0 0 0] Plays Lights out sound
  (CallFunction|PlayUISoundEffect "/Game/TwentyItems/Sound/Temporary/LightsOut_Cue.LightsOut_Cue" 0 1.0)
  ;;[0 0 0] Gets Starting sky light intensity
  (Variables|LightsOut|SetStartingSkyLightIntensity (Variables|/Script/Engine.LightComponentBase|GetIntensity (Variables|/Script/Engine.SkyLight|GetLightComponent (References|GetSkyLightRef))))
  ;;[0 0 0] Sets How Long it takes to turn off the lights
  (Components|Timeline|SetPlayRate (Variables|Default|GetLightsOutTimeLine) (/ 1.0 (Variables|LightsOut|GetLightsOutTransitionTime)))
  (Variables|LightsOut|SetPlayingLightsOutTimeline? true)
  (bind _skylightintensityalpha (Timeline|LightsOutTimeLine PlayFromStart)
    (:Update
      (Rendering|Components|Light|SetIntensity (Variables|/Script/Engine.SkyLight|GetLightComponent (References|GetSkyLightRef)) (Math|Float|Lerp (Variables|LightsOut|GetLightsOutSkyLightIntensity) (Variables|LightsOut|GetStartingSkyLightIntensity) _skylightintensityalpha)))
    (:Finished
      ;;[0 0 0] Used for clients who weren't in the game when the multicast event was called to turn off lights
      (Variables|LightsOut|SetPlayingLightsOutTimeline? false)
      (Networking|SwitchHasAuthority
        (:Authority
          (Variables|LightsOut|SetTurnedLightsOff true))))))

(event Custom|PlayVictoryEffects
  ;[1 0 0] Play Victory Effects
  (CallFunction|PlayUISoundEffect (Variables|EndGameEffects|GetVictorySoundEffect) 0 1.0)
  (bind _returnvalue (UserInterface|CreateWidget "/Game/TwentyItems/Blueprints/Player/UI/GameState/GameMode/VictoryScreen.VictoryScreen_C"))
  (UserInterface|Viewport|AddtoViewport _returnvalue 0))

(fn ConstructionScript)

(fn OnRepPreparingtoStartGame)

(fn OnRepMatchState
  (switch int (Variables|MatchState|GetMatchState%20)
    (:1
      (MatchState|StartCountDownTimer))
    (:2
      (MatchState|StartPreparationPhase))))

(fn StartCountDownTimer)

(fn StartPreparationPhase
  (bind _returnvalue (UserInterface|CreateWidget "/Game/TwentyItems/Blueprints/Player/UI/GameState/GameMode/W_StartPreparations.W_StartPreparations_C" (Game|GetPlayerController 0)))
  (UserInterface|Viewport|AddtoViewport _returnvalue 0))

(fn GetControllerRef)

(fn GetSkyLightRef
  (Utilities|IsValid (Variables|References|GetSkyLightRef)
    (:Is%20Valid
      _)
    (:Is%20Not%20Valid
      (bind _outactors (Actor|GetAllActorsOfClass "/Script/Engine.SkyLight"))
      (bind _output_get (Variables|References|SetSkyLightRef (Utilities|Array|Get(acopy) _outactors)))))
  (return _output_get))

(fn OnRepTurnedLightsOff
  (if (and (not (Variables|LightsOut|GetPlayingLightsOutTimeline?)) (Variables|LightsOut|GetTurnedLightsOff))
    (Rendering|Components|Light|SetIntensity (Variables|/Script/Engine.SkyLight|GetLightComponent (References|GetSkyLightRef)) (Variables|LightsOut|GetLightsOutSkyLightIntensity))))