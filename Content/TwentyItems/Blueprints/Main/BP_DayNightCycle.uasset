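; Day-night cycle actor that pitches a Sun actor toward a target angle over a set transition time and refreshes the SkyDome's sun direction.
; Tick advances the angle at a derived speed, clamped between zero and the target, while construction previews it.
; RepNotifies on target angle and time recompute that speed.
; The authority records ServerSunAngle; despite its name, ClientRequestSunAngle applies it only on authority at BeginPlay.
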(event EventBeginPlay
  ;[1 0 0] Event Begin Play
  ;;[1 1 1] When a client spawns in he can sync his sun with the server
  (CallFunction|ClientRequestSunAngle)
  (CallFunction|UpdateSunTarget))

(event EventTick
  (params (DeltaSeconds :type Float%20%28single-precision%29))
  (Variables|Default|SetCurrentSunAngle (Math|Float|Clamp(Float) (+ (* DeltaSeconds (Variables|Default|GetTransitionSpeed)) (Variables|Default|GetCurrentSunAngle)) 0.0 (Variables|Default|GetTargetSunAngle)))
  (CallFunction|SetSunAngle (Variables|Default|GetCurrentSunAngle)))

(fn ConstructionScript
  (if (and (Utilities|IsValid (Variables|Default|GetSun)) (Utilities|IsValid (Variables|Default|GetSkyDome)))
    (Transformation|SetActorRotation (Variables|Default|GetSun) (Math|Rotator|MakeRotator 0.0 (Variables|Default|GetCurrentSunAngle) 0.0))
    (Default|UpdateSunDirection (Variables|Default|GetSkyDome))))

(fn SetSunAngle
  (params (New%20Angle :type Float%20%28single-precision%29))
  (Variables|Default|SetCurrentSunAngle New%20Angle)
  (Transformation|SetActorRotation (Variables|Default|GetSun) (Math|Rotator|MakeRotator 0.0 New%20Angle 0.0))
  (Default|UpdateSunDirection (Variables|Default|GetSkyDome))
  (Networking|SwitchHasAuthority
    (:Authority
      (Variables|Default|SetServerSunAngle (Variables|Default|GetCurrentSunAngle)))))

(fn ClientRequestSunAngle
  (Networking|SwitchHasAuthority
    (:Authority
      (CallFunction|SetSunAngle (Variables|Default|GetServerSunAngle)))))

(fn UpdateSunTarget
  (Variables|Default|SetTransitionSpeed (/ (- (Variables|Default|GetTargetSunAngle) (Variables|Default|GetCurrentSunAngle)) (Variables|Default|GetTargetTimeTransition))))

(fn OnRepTargetTimeTransition
  (CallFunction|UpdateSunTarget))

(fn OnRepTargetSunAngle
  (CallFunction|UpdateSunTarget))