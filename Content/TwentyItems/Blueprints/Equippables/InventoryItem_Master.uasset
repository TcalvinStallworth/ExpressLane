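; Base pickup actor for equippable inventory items, configured from a data table row looked up by its DataKey.
; On BeginPlay the server caches the row's slot info, fills an empty stack with the default amount and rolls a random combine ID.
; The construction script writes rarity to the mesh's custom depth stencil for glow color.
; Hovering updates the player's interact message widget, and pickup plays the row's UI sound cue.
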(event EventBeginPlay
  (bind _datakey_ (Variables|SlotInfo|GetDataKey%20))
  (bind (_data _foundrow_) (CallFunction|GetEquippableDatafromTable _datakey_))
  ;[1 1 1] Event Begin Play | finds item on data table and sets random combine ID
  (Networking|SwitchHasAuthority
    (:Authority
      (bind _output_get (Variables|SlotInfo|SetSlotInfo%20 (select _foundrow_ _data (Variables|SlotInfo|GetSlotInfo%20))))
      (Utilities|FlowControl|Sequence
        (:then_0
          (if (== (Variables|Combining|GetStackAmount) 0)
            (Variables|Combining|SetStackAmount (.DefaultStack (Utilities|Struct|BreakEquippableInventoryStruct _output_get)))))
        (:then_1
          (Variables|Combining|SetRandomCombineID (Math|Random|RandomFloatinRange 0.0 1e+06)))))))

(event EventHovered
  (params (Player%20Controller :type Player%20Controller%20Object%20Reference) (Hit%20Result :type Hit%20Result%20Structure) (Character :type Express%20Lane%20Character%20Object%20Reference))
  ;[1 1 1] Event Hovered
  (Variables|/Game/TwentyItems/Blueprints/Player/ExpressLaneCharacter.ExpressLaneCharacter_C|SetWidgetSwitcherIndex Character 0)
  (Default|UpdateInteractMessage (Variables|/Game/TwentyItems/Blueprints/Main/Skylands/PC_ExpressLane.PC_ExpressLane_C|GetInteractMessageWidget (Default|GetPlayerControllerClient Character)) self (Variables|SlotInfo|GetDataKey%20)))

(fn ConstructionScript
  ;[1 1 1] Glow Color
  (Rendering|SetCustomDepthStencilValue (Variables|Default|GetStaticMesh) (+ (Math|Conversions|ToInteger(Byte) (.Rarity (Utilities|Struct|BreakEquippableInventoryStruct (.Data (CallFunction|GetEquippableDatafromTable (Variables|SlotInfo|GetDataKey%20)))))) 1)))

(fn PlayPickUpEffects
  (params (Character :type Express%20Lane%20Character%20Object%20Reference))
  (CallFunction|PlayUISoundEffect (.PickUpCue (Utilities|Struct|BreakEquippableInventoryStruct (.Data (CallFunction|GetEquippableDatafromTable (Variables|SlotInfo|GetDataKey%20))))) Character 1.0))