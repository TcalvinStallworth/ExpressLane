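; Server-only pickup spawner that places one random lootable at its spawn point on BeginPlay, then destroys itself.
; It rolls a category from weighted tickets, then an item by SpawnRate from GM_ExpressLaneOLD's filtered loot list.
; Both cumulative-weight rolls use the procedural level manager's seeded stream when GeneratedSeed is true.
; SpawnItem handles equippables and ammo, but selection always passes the Item type, leaving the ammo branch unused.
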(event EventBeginPlay
  (Networking|SwitchHasAuthority
    (:Authority
      (bind _asgm_express_lane_old (Utilities|Casting|CastToGM_ExpressLaneOLD (Game|GetGameMode)))
      (Variables|Default|SetGM_ExpressLane _asgm_express_lane_old)
      (CallFunction|SelectSpawningCategory)
      (CallFunction|SelectSpawnedItem))))

(fn ConstructionScript)

(fn SelectSpawnedItem
  (bind _itemspawntype (Variables|Default|GetItemSpawnType))
  (bind _gm_expresslane (Variables|Default|GetGM_ExpressLane))
  (bind (_matching_structs _tallies) (Default|FilterItemPickUpSpawnerLootables _gm_expresslane _itemspawntype))
  (bind _procedurallevelmanager (Default|GetProceduralLevelManagerRef _gm_expresslane))
  (Networking|SwitchHasAuthority
    (:Authority
      (LocalVariables|SetSelectionAddition 0)
      ;[1 1 1] Selects the index to spawn item
      (LocalVariables|SetSpawnedIndex (select (Variables|/Game/TwentyItems/Blueprints/ProceduralGeneration/ProceduralLevelManager.ProceduralLevelManager_C|GetGeneratedSeed? _procedurallevelmanager) (Math|Random|RandomIntegerinRangefromStream 0 _tallies (Variables|/Game/TwentyItems/Blueprints/ProceduralGeneration/ProceduralLevelManager.ProceduralLevelManager_C|GetRandomSeed _procedurallevelmanager)) (Math|Random|RandomIntegerinRange 0 _tallies)))
      (bind _array_element (Utilities|Array|ForEachLoopwithBreak _matching_structs :!label _label)
        (:LoopBody
          (bind _output_get (LocalVariables|SetSelectionAddition (+ (.SpawnRate (Utilities|Struct|BreakLootable_Struct _array_element)) (LocalVariables|GetSelectionAddition))))
          (if (not (> (LocalVariables|GetSpawnedIndex) _output_get))
            (CallFunction|SpawnItem (.Actor (Utilities|Struct|BreakLootable_Struct _array_element)) "NewEnumerator0")
            (goto _label Break)))))))

(fn SpawnItem
  (params (Item :type Actor%20Class%20Reference) (ItemType :type InventoryItemType%20Enum :default "NewEnumerator0"))
  (bind _spawnpoint (Variables|Default|GetSpawnPoint))
  (bind _returnvalue (Transformation|GetWorldTransform _spawnpoint))
  (Networking|SwitchHasAuthority
    (:Authority
      (LocalVariables|SetItemSpawning Item)
      (Utilities|FlowControl|Sequence
        (:then_0
          (bind _output_get (LocalVariables|SetItem%20Type ItemType))
          (switch Utilities|FlowControl|Switch|SwitchonInventoryItemType _output_get
            (:NewEnumerator0
              (bind _asequippable_parent (Utilities|Casting|CastToEquippableParentClass (LocalVariables|GetItemSpawning)))
              (Utilities|SpawnItem _asequippable_parent _returnvalue))
            (:NewEnumerator1
              (bind _asammo_pickup_parent (Utilities|Casting|CastToAmmoPickupParentClass (LocalVariables|GetItemSpawning)))
              (Utilities|SpawnAmmo _asammo_pickup_parent _returnvalue))))
        (:then_1
          ;[1 1 1] Actor is destroyed after spawning item
          (Actor|DestroyActor))))))

(fn SelectSpawningCategory
  (bind _gm_expresslane (Variables|Default|GetGM_ExpressLane))
  (bind _procedurallevelmanager (Default|GetProceduralLevelManagerRef _gm_expresslane))
  (Networking|SwitchHasAuthority
    (:Authority
      (bind _values (Utilities|Map|Values (Variables|Default|GetItemTypeSpawnTickets)))
      (for _array_element _values
        (LocalVariables|SetTallies (+ _array_element (LocalVariables|GetTallies))))
      (LocalVariables|SetRandomSelection (select (Variables|/Game/TwentyItems/Blueprints/ProceduralGeneration/ProceduralLevelManager.ProceduralLevelManager_C|GetGeneratedSeed? _procedurallevelmanager) (Math|Random|RandomIntegerinRangefromStream 0 (LocalVariables|GetTallies) (Variables|/Game/TwentyItems/Blueprints/ProceduralGeneration/ProceduralLevelManager.ProceduralLevelManager_C|GetRandomSeed _procedurallevelmanager)) (Math|Random|RandomIntegerinRange 0 (LocalVariables|GetTallies))))
      (bind _keys (Utilities|Map|Keys (Variables|Default|GetItemTypeSpawnTickets)))
      (bind _array_element_2 (Utilities|Array|ForEachLoopwithBreak _keys :!label _label)
        (:LoopBody
          (bind _output_get (LocalVariables|SetSelectionAddition (+ (.Value (Utilities|Map|Find (Variables|Default|GetItemTypeSpawnTickets) _array_element_2)) (LocalVariables|GetSelectionAddition))))
          (if (not (> (LocalVariables|GetRandomSelection) _output_get))
            (Variables|Default|SetItemSpawnType _array_element_2)
            (goto _label Break)))))))