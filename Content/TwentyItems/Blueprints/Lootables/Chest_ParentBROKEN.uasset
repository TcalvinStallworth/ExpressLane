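; Searchable loot chest parent that a player opens by holding view on it until a progress timer completes.
; Activate starts a looping timer that line-traces each step, cancelling on lost sight, while controller-relayed client events toggle the progress widget.
; Completion triggers effects, a replicated mesh swap, and authority-only spawning of money plus weighted-random consumable and weapon, thrown toward the looter.
; Controller casts have no target class, matching the BROKEN name.
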(event Custom|PlaySearchEffects
  (bind _returnvalue (Transformation|GetActorRotation))
  (bind _spawnpoint (Variables|Default|GetSpawnPoint))
  (bind _returnvalue_2 (Transformation|GetWorldLocation _spawnpoint))
  ;[1 1 1] Play Search Effects
  ;;[1 1 1] Plays Open Sound Effects
  (CallFunction|PlaySoundatLocationFunction (Variables|FX|GetBoxOpenSound) _returnvalue_2 _returnvalue (.AsExpress%20Lane%20Game%20Instance (Utilities|Casting|CastToExpressLane_GameInstance (Game|GetGameInstance))) "NewEnumerator0")
  ;;[1 1 1] Plays Emitter
  (Effects|SpawnEmitteratLocation 0 (Variables|FX|GetBoxOpenParticle) _returnvalue_2 _returnvalue))

(event Collision|EventActorBeginOverlap
  (params (OtherActor :type Actor%20Object%20Reference)))

(event EventActivate
  (params (Player%20Controller :type Player%20Controller%20Object%20Reference) (Hit%20Result :type Hit%20Result%20Structure) (Character :type Express%20Lane%20Character%20Object%20Reference))
  ;[1 1 1] Event Activate
  ;;[1 1 1] Makes sure the lootable isn't already being searched and it's not already been searched
  (if (and (not (Variables|Looting|GetLooted?)) (not (Variables|Looting|GetBeingSearched?)))
    ;;[1 1 1] Tells client to create widget
    (bind _aspc_express_lane (Utilities|Casting|CastTo Player%20Controller))
    (CallFunction|CallClientEvent _aspc_express_lane self)
    ;;[1 1 1] Starts Searching
    (CallFunction|StartSearching Character)))

(event EventCallClientEvent
  (params (Event :type Integer))
  ;[1 1 1] Client Event
  (switch int Event
    (:0
      (ClientEvents|ClientEvent0))
    (:1
      (ClientEvents|ClientEvent1))))

(event EventCancelInteract
  ;[1 1 1] Interact Cancelled
  (CallFunction|CancelSearching))

(fn ConstructionScript)

(fn OnRepLooted?
  (bind _lootedmesh (Variables|Default|GetLootedMesh))
  (if (Variables|Looting|GetLooted?)
    ;[1 1 1] Destroys the looted mesh
    (Components|DestroyComponent (Variables|Default|GetUnlootedMesh))
    ;[1 1 1] Unhides the looted mesh
    (Development|SetHiddeninGame _lootedmesh false false)
    ;[1 1 1] Re-enables collision
    (Collision|SetCollisionEnabled _lootedmesh "QueryAndPhysics")
    (Components|DestroyComponent (Variables|Default|GetIdleSound))))

(fn StartSearching
  (params (InteractingCharacter :type Express%20Lane%20Character%20Object%20Reference))
  (Variables|Looting|SetInteractingCharacter InteractingCharacter)
  ;[1 1 1] Tells the character he's interacting with something
  (Variables|/Game/TwentyItems/Blueprints/Player/ExpressLaneCharacter.ExpressLaneCharacter_C|SetInteractingDown? (Variables|Looting|GetInteractingCharacter) true)
  (Variables|/Game/TwentyItems/Blueprints/Player/ExpressLaneCharacter.ExpressLaneCharacter_C|SetInteractedActor (Variables|Looting|GetInteractingCharacter) self)
  ;[1 1 1] Sets Being Searched To True
  (Variables|Looting|SetBeingSearched? true)
  ;[1 1 1] Sets timer to update loot progress
  (bind _returnvalue (Utilities|Time|SetTimerbyFunctionName 0 "UpdateLootProgress" 0.1 true))
  (Variables|Looting|SetLootProgressTimer _returnvalue))

(fn CancelSearching
  (if (Variables|Looting|GetBeingSearched?)
    ;[1 1 1] Tells client to Remove widget
    (bind _aspc_express_lane (Utilities|Casting|CastTo (Pawn|GetController (Variables|Looting|GetInteractingCharacter))))
    (CallFunction|CallClientEvent _aspc_express_lane self 1)
    ;[1 1 1] Clears interacting character and sets being searched to false
    (Variables|Looting|SetInteractingCharacter 0)
    (Variables|Looting|SetBeingSearched? false)
    ;[1 1 1] Resets Loot Progress
    (Variables|Looting|SetLootedProgress 0.0)
    ;[1 1 1] Clears loot progress timer
    (Utilities|Time|ClearandInvalidateTimerbyHandle 0 (Variables|Looting|GetLootProgressTimer))))

(fn ClientEvent0
  (bind _aspc_express_lane (Utilities|Casting|CastTo (Game|GetPlayerController 0)))
  (CallFunction|CreateLootableWidget _aspc_express_lane self))

(fn ClientEvent1
  ;[1 1 1] Tells client to Remove widget
  (bind _aspc_express_lane (Utilities|Casting|CastTo (Game|GetPlayerController 0)))
  (CallFunction|RemoveLootableWidget _aspc_express_lane))

(fn UpdateLootProgress
  (bind _can_loot_ (CallFunction|ShouldCancelLooting?))
  (if _can_loot_
    ;[1 1 1] Increments loot progress
    (bind _output_get (Variables|Looting|SetLootedProgress (+ (Variables|Looting|GetLootedProgress) 0.1)))
    ;[1 1 1] Checks if the loot bar is full
    (if (>= _output_get (Variables|Looting|GetLootTime))
      (CallFunction|FinishLooting))
    (else
      (CallFunction|CancelSearching))))

(fn FinishLooting
  ;[1 1 1] Updates Mesh
  (Variables|Looting|SetLooted? true)
  ;[1 1 1] Spawns the Loot
  (Spawning|SpawnLoot)
  ;[1 1 1] Cancels looting and removes widget
  (CallFunction|CancelSearching)
  ;[1 1 1] Plays effects to relevant players
  (CallFunction|PlaySearchEffects))

(fn ShouldCancelLooting?
  (bind _interactingcharacter (Variables|Looting|GetInteractingCharacter))
  (bind _firstpersoncamera (Variables|/Game/TwentyItems/Blueprints/Player/ExpressLaneCharacter.ExpressLaneCharacter_C|GetFirstPersonCamera _interactingcharacter))
  (bind _returnvalue (Transformation|GetWorldLocation _firstpersoncamera))
  ;[1 1 1] Checks if you are still allowed to interact
  (if (Variables|/Game/TwentyItems/Blueprints/Player/ExpressLaneCharacter.ExpressLaneCharacter_C|GetInteractAllowed? _interactingcharacter)
    (bind (_outhit _returnvalue_2) (Collision|LineTraceByChannel 0 _returnvalue (+ _returnvalue (* (Math|Vector|GetForwardVector (Variables|/Game/TwentyItems/Blueprints/Player/ExpressLaneCharacter.ExpressLaneCharacter_C|GetControlRotation _interactingcharacter)) (Variables|/Game/TwentyItems/Blueprints/Player/ExpressLaneCharacter.ExpressLaneCharacter_C|GetInteractDistance _interactingcharacter))) "TraceTypeQuery1" false (Utilities|Array|MakeArray _interactingcharacter (Default|GetEquippedItem _interactingcharacter)) "ForDuration" false))
    (if _returnvalue_2
      (if (== (.HitActor (Collision|BreakHitResult _outhit)) self)
        (LocalVariables|SetCanLoot? true)
        (else
          (bind _output_get (LocalVariables|SetCanLoot? false :!label _label))))
      (else
        (goto _label)))
    (else
      (LocalVariables|SetCanLoot? false)))
  (return _output_get))

(fn SpawnLoot
  (Spawning|SpawnConsumable)
  (Spawning|SpawnWeapon)
  (Spawning|SpawnMoney))

(fn SpawnConsumable
  (Networking|SwitchHasAuthority
    (:Authority
      (bind (_matching_structs _tallies) (CallFunction|FilterSpawnableLootbyItemTypes (Variables|Default|GetLootDataKey) (Utilities|Array|MakeArray "NewEnumerator1" "NewEnumerator3" "NewEnumerator5")))
      (LocalVariables|SetFilteredConsumables _matching_structs)
      (LocalVariables|SetTotalTallies _tallies)
      (LocalVariables|SetSelectionAddition 0)
      ;[1 1 1] Selects the index to spawn item
      (LocalVariables|SetSpawnedIndex (Math|Random|RandomIntegerinRange 1 (LocalVariables|GetTotalTallies)))
      ;[1 1 1] Selects Item to spawn
      (bind _array_element (Utilities|Array|ForEachLoopwithBreak (LocalVariables|GetFilteredConsumables) :!label _label)
        (:LoopBody
          (bind _output_get (LocalVariables|SetSelectionAddition (+ (.SpawnRate (Utilities|Struct|BreakLootable_Struct _array_element)) (LocalVariables|GetSelectionAddition))))
          (if (not (> (LocalVariables|GetSpawnedIndex) _output_get))
            (Spawning|SpawnItem (.Actor (Utilities|Struct|BreakLootable_Struct _array_element)))
            (goto _label Break)))))))

(fn SpawnItem
  (params (Spawned%20Actor :type Actor%20Class%20Reference))
  (bind _returnvalue (Transformation|GetActorLocation))
  (bind _spawndistancedeviation (Variables|Spawning|GetSpawnDistanceDeviation))
  (bind _spawndirectiondeviation (Variables|Spawning|GetSpawnDirectionDeviation))
  (bind _interactingcharacter (Variables|Looting|GetInteractingCharacter))
  (bind _spawnlocationdeviation (Variables|Spawning|GetSpawnLocationDeviation))
  (bind _spawnpoint (Variables|Default|GetSpawnPoint))
  (bind _spawndistance (Variables|Spawning|GetSpawnDistance))
  (bind _returnvalue_2 (Transformation|GetWorldTransform _spawnpoint))
  (bind _returnvalue_3 (/ _spawnlocationdeviation 2.0))
  (bind _returnvalue_4 (Transformation|GetActorLocation _interactingcharacter))
  (bind _returnvalue_5 (* _spawndirectiondeviation -1.0))
  (bind _returnvalue_6 (* _spawndistancedeviation -1.0))
  (bind _returnvalue_7 (+ _spawndistance _spawndistancedeviation))
  (bind (_location _rotation _scale) (Math|Transform|BreakTransform _returnvalue_2))
  (bind _returnvalue_8 (Math|Rotator|FindLookatRotation _returnvalue_4 _returnvalue))
  (bind _returnvalue_9 (Math|Random|RandomFloatinRange _returnvalue_5 _spawndirectiondeviation))
  (bind _returnvalue_10 (Math|Random|RandomFloatinRange _returnvalue_5 _spawndirectiondeviation))
  (bind _returnvalue_11 (Math|Random|RandomFloatinRange _returnvalue_5 _spawndirectiondeviation))
  (bind _returnvalue_12 (* _returnvalue_3 -1.0))
  (bind _returnvalue_13 (+ _spawndistance _returnvalue_6))
  (bind (_roll _pitch) (Math|Rotator|BreakRotator _rotation))
  (bind _returnvalue_14 (Math|Vector|GetForwardVector _returnvalue_8))
  (bind (_x _y _z) (Math|Vector|BreakVector _location))
  (bind _returnvalue_15 (Math|Random|RandomFloatinRange _returnvalue_13 _returnvalue_7))
  (bind (_x_2 _y_2 _z_2) (Math|Vector|BreakVector _returnvalue_14))
  (bind _returnvalue_16 (+ _z_2 _returnvalue_9))
  (bind _returnvalue_17 (+ _x_2 _returnvalue_10))
  (bind _returnvalue_18 (+ _y_2 _returnvalue_11))
  (bind _returnvalue_19 (Math|Vector|MakeVector _returnvalue_17 _returnvalue_18 _returnvalue_16))
  (bind _returnvalue_20 (* _returnvalue_19 -1.0))
  (bind (_x_3 _y_3) (Math|Vector|BreakVector _returnvalue_20))
  (bind _returnvalue_21 (Math|Vector|MakeVector _x_3 _y_3 0.2))
  (bind _returnvalue_22 (* _returnvalue_21 _returnvalue_15))
  (Networking|SwitchHasAuthority
    (:Authority
      (bind _asinventory_item_master (Utilities|Casting|CastToInventoryItem_MasterClass Spawned%20Actor))
      (bind (_spawneditem _spawnedammo) (Utilities|SpawnItem _asinventory_item_master (Math|Transform|MakeTransform (Math|Vector|MakeVector (+ _x (Math|Random|RandomFloatinRange _returnvalue_12 _returnvalue_3)) (+ _y (Math|Random|RandomFloatinRange _returnvalue_12 _returnvalue_3)) (+ _z (Math|Random|RandomFloatinRange _returnvalue_12 _returnvalue_3))) (Math|Rotator|MakeRotator _roll _pitch (Math|Random|RandomFloatinRange -1.8e+02 1.8e+02)) _scale))
        (:%20
          (LocalVariables|SetEquippableRef _spawneditem)
          (LocalVariables|SetSpawnedAmmo _spawnedammo)
          ;[0 0 0] Spawns Mesh
          (Physics|AddImpulse (Variables|/Game/TwentyItems/Blueprints/Equippables/InventoryItem_Master.InventoryItem_Master_C|GetSphere%20Collision (LocalVariables|GetEquippableRef)) _returnvalue_22 "None" true)
          ;[0 0 0] Ammo Impulse
          (Utilities|IsValid (LocalVariables|GetSpawnedAmmo)
            (:Is%20Valid
              (bind _asammo_pickup_parent (Utilities|Casting|CastToAmmoPickupParent (LocalVariables|GetSpawnedAmmo)))
              (Physics|AddImpulse (Variables|/Game/TwentyItems/Blueprints/Equippables/InventoryItem_Master.InventoryItem_Master_C|GetSphere%20Collision _asammo_pickup_parent) _returnvalue_22 "None" true))))))))

(fn SpawnWeapon
  (Networking|SwitchHasAuthority
    (:Authority
      (bind (_matching_structs _tallies) (CallFunction|FilterSpawnableLootbyItemTypes (Variables|Default|GetLootDataKey) (Utilities|Array|MakeArray "NewEnumerator2" "NewEnumerator0")))
      (LocalVariables|SetFilteredWeapons _matching_structs)
      (LocalVariables|SetTotalTallies _tallies)
      (LocalVariables|SetSelectionAddition 0)
      ;[1 1 1] Selects the index to spawn item
      (LocalVariables|SetSpawnedIndex (Math|Random|RandomIntegerinRange 1 (LocalVariables|GetTotalTallies)))
      ;[1 1 1] Selects Item to spawn
      (bind _array_element (Utilities|Array|ForEachLoopwithBreak (LocalVariables|GetFilteredWeapons) :!label _label)
        (:LoopBody
          (bind _output_get (LocalVariables|SetSelectionAddition (+ (.SpawnRate (Utilities|Struct|BreakLootable_Struct _array_element)) (LocalVariables|GetSelectionAddition))))
          (if (not (> (LocalVariables|GetSpawnedIndex) _output_get))
            (Spawning|SpawnItem (.Actor (Utilities|Struct|BreakLootable_Struct _array_element)))
            (goto _label Break)))))))

(fn SpawnMoney
  (Networking|SwitchHasAuthority
    (:Authority
      (Spawning|SpawnItem "/Game/TwentyItems/Blueprints/Lootables/Pickups/Money/MoneyPickUp.MoneyPickUp_C"))))