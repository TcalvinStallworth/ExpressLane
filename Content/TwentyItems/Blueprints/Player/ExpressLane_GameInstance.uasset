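; Game instance that holds player settings, Cognito auth tokens and online session flow.
; Init loads sound, gameplay, control and Fagoozle gun settings from a save slot, with a matching function to write them back.
; Joining or leaving a match destroys the current session first, then proceeds even if that fails; session creation events are empty.
; Also refreshes tokens through Cognito, calls Destroy on server shutdown, prints network errors and tracks gamepad use.
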(event Custom|CreateSession)

(event Custom|JoinSession
  (params (Session :type Blueprint%20Session%20Result%20Structure) (TeamID :type String))
  (bind _returnvalue (Game|GetPlayerController 0))
  (Variables|Default|SetTeamID TeamID)
  (Variables|Default|SetSessionDELETE Session)
  (|DestroySession _returnvalue
    (:then
      (Development|PrintString "JOINING SESSION"))
    (:OnSuccess
      (|JoinSession _returnvalue (Variables|Default|GetSessionDELETE) :!label _label))
    (:OnFailure
      (goto _label))))

(event Custom|CreateInitSession
  ;[1 1 1] Create Init Session
)

(event Custom|LeaveMatch
  (|DestroySession (Game|GetPlayerController 0)
    (:then
      ;[1 1 1] Create Init Session
      (Development|PrintString "LEAVING MATCH" true true "(R=0.000000,G=0.660000,B=1.000000,A=1.000000)" 1e+01))
    (:OnSuccess
      (CallFunction|OpenLevel :!label _label))
    (:OnFailure
      (goto _label))))

(event Custom|OpenLevel
  (Game|OpenLevel(byName) "EntryMap" true "?listen"))

(event Custom|SwitchInputDevice
  (params (Is%20GamePad%20Input? :type Boolean))
  ;[1 1 1] Switch Input Device
  (Variables|Settings|SetUsingGamepad? Is%20GamePad%20Input?))

(event Custom|RefrashToken
  (bind (_success _initiateauthresult _errortype _errormessage) (Class|CognitoIdpClientObject|InitiateAuth (Variables|Default|GetCognito%20IDP%20Client) (Utilities|Struct|MakeInitiateAuthRequest "REFRESH_TOKEN" (Utilities|Map|MakeMap "REFRESH_TOKEN" (Variables|Default|GetRefreshToken)) (Utilities|Map|MakeMap) (Variables|AWSSetup|GetClient%20ID))))
  (if _success
    (switch Utilities|FlowControl|Switch|SwitchonEChallengeNameType (.challengeName (Utilities|Struct|BreakInitiateAuthResult _initiateauthresult))
      (:NOT_SET
        (Variables|Default|SetAccessToken (.accessToken (Utilities|Struct|BreakAuthenticationResultType (.authenticationResult (Utilities|Struct|BreakInitiateAuthResult _initiateauthresult)))))
        (Variables|Default|SetRefreshToken (.refreshToken (Utilities|Struct|BreakAuthenticationResultType (.authenticationResult (Utilities|Struct|BreakInitiateAuthResult _initiateauthresult)))))
        (Variables|Default|SetIdToken (.idToken (Utilities|Struct|BreakAuthenticationResultType (.authenticationResult (Utilities|Struct|BreakInitiateAuthResult _initiateauthresult)))))))
    (else
      (Development|PrintString _errormessage))))

(event EventInit
  ;[1 0 0] Event Init
  (Settings|LoadGameSettings))

(event EventHandleNetworkError
  (params (FailureType :type ENetworkFailure%20Enum :default "NetDriverAlreadyExists") (bIsServer :type Boolean))
  (Development|PrintString (Utilities|String|EnumtoString FailureType) true true "(R=1.000000,G=1.000000,B=0.000000,A=1.000000)" 1e+01))

(event EventShutdown
  ;[0 0.5 0.4797] Event Shutdown
  (if (Networking|IsServer)
    (bind (_success _errortype _errormessage) (Class|GameLiftServerFunctionLibrary|Destroy))
    (if _success
      (Development|PrintString "YouDestroyed")
      (else
        (Development|PrintString _errormessage)))))

(fn SaveGameSettings
  (Utilities|IsValid (Variables|Saves|GetSettingsSaveInstance)
    (:Is%20Valid
      _)
    (:Is%20Not%20Valid
      (bind _returnvalue (SaveGame|CreateSaveGameObject "/Game/TwentyItems/Blueprints/Player/Settings/SaveGames/SaveGameSettings.SaveGameSettings_C"))
      (Variables|Saves|SetSettingsSaveInstance _returnvalue)))
  ;[1 1 1] Creates Save Game and Saves it
  (Variables|/Game/TwentyItems/Blueprints/Player/Settings/SaveGames/SaveGameSettings.SaveGameSettings_C|SetSoundSettings (Variables|Saves|GetSettingsSaveInstance) (Variables|Settings|GetSoundSettings))
  (Variables|/Game/TwentyItems/Blueprints/Player/Settings/SaveGames/SaveGameSettings.SaveGameSettings_C|SetGameplaySettings (Variables|Saves|GetSettingsSaveInstance) (Variables|Settings|GetGameplaySettings))
  (Variables|/Game/TwentyItems/Blueprints/Player/Settings/SaveGames/SaveGameSettings.SaveGameSettings_C|SetControlSettings (Variables|Saves|GetSettingsSaveInstance) (Variables|Settings|GetControlSettings))
  (Variables|/Game/TwentyItems/Blueprints/Player/Settings/SaveGames/SaveGameSettings.SaveGameSettings_C|SetFagoozleGunSettings (Variables|Saves|GetSettingsSaveInstance) (Variables|Settings|GetFagoozleGunSettings))
  (SaveGame|SaveGametoSlot (Variables|Saves|GetSettingsSaveInstance) "GameSettings"))

(fn LoadGameSettings
  ;[1 1 1] Checks if the game settings exist
  (bind _returnvalue (SaveGame|DoesSaveGameExist "GameSettings"))
  (if _returnvalue
    ;[1 1 1] If the game settings do exist they are loaded in
    (bind _returnvalue_2 (SaveGame|LoadGamefromSlot "GameSettings"))
    (bind _assave_game_settings (Utilities|Casting|CastToSaveGameSettings _returnvalue_2))
    ;[1 1 1] Loads up Your Settings
    (Variables|Settings|SetSoundSettings (Variables|/Game/TwentyItems/Blueprints/Player/Settings/SaveGames/SaveGameSettings.SaveGameSettings_C|GetSoundSettings _assave_game_settings))
    (Variables|Settings|SetControlSettings (Variables|/Game/TwentyItems/Blueprints/Player/Settings/SaveGames/SaveGameSettings.SaveGameSettings_C|GetControlSettings _assave_game_settings))
    (Variables|Settings|SetFagoozleGunSettings (Variables|/Game/TwentyItems/Blueprints/Player/Settings/SaveGames/SaveGameSettings.SaveGameSettings_C|GetFagoozleGunSettings _assave_game_settings))
    (Variables|Settings|SetGameplaySettings (Variables|/Game/TwentyItems/Blueprints/Player/Settings/SaveGames/SaveGameSettings.SaveGameSettings_C|GetGameplaySettings _assave_game_settings))))