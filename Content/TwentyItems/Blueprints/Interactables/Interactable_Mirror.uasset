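; Interactable mirror whose glass fogs up when fog is added and gradually clears on its own.
; BeginPlay creates a dynamic instance of the glass material on the mirror mesh.
; AddFogValue adds scaled, clamped fog, while Tick interpolates it back toward zero.
; Each tick maps the fog amount onto the material's minimum and maximum roughness, blending between clear and fully fogged ranges.
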(event Custom|AddFogValue
  (params (Value :type Float%20%28single-precision%29))
  ;[1 1 1] Add Fog Value
  (Variables|Default|SetFogValue (Math|Float|Clamp(Float) (+ (* Value (Variables|Default|GetAddFogScale)) (Variables|Default|GetFogValue)))))

(event EventBeginPlay
  ;[1 1 1] Creates DMI
  (|CallParentFunction)
  (bind _returnvalue (Rendering|Material|CreateDynamicMaterialInstance (Variables|Default|GetMirror) 1 "/Game/TwentyItems/Materials/PROTO/Testglass_Inst.Testglass_Inst" "None" :!class /Script/Engine.PrimitiveComponent))
  (Variables|Default|SetDMI _returnvalue))

(event EventTick
  (params (DeltaSeconds :type Float%20%28single-precision%29))
  (bind _dmi (Variables|Default|GetDMI))
  (bind _nofogroughnessrange (Variables|Default|GetNoFogRoughnessRange))
  (bind _maxfogroughnessrange (Variables|Default|GetMaxFogRoughnessRange))
  (|CallParentFunction DeltaSeconds)
  ;[0 0 0] Sets Fog
  (Rendering|Material|SetScalarParameterValue _dmi "RoughnessMax" (Math|Float|Lerp (.x _nofogroughnessrange) (.x _maxfogroughnessrange) (Variables|Default|GetFogValue)) :!class /Script/Engine.MaterialInstanceDynamic)
  (Rendering|Material|SetScalarParameterValue _dmi "RoughnessMin" (Math|Float|Lerp (.y _nofogroughnessrange) (.y _maxfogroughnessrange) (Variables|Default|GetFogValue)) :!class /Script/Engine.MaterialInstanceDynamic)
  (Variables|Default|SetFogValue (Math|Interpolation|FInterpTo (Variables|Default|GetFogValue) 0.0 DeltaSeconds (Variables|Default|GetDefogInterpSpeed))))

(fn ConstructionScript
  (|CallParentFunction))