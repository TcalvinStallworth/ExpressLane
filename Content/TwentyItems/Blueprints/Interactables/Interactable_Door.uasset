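; Interactable door that players toggle open and closed, with the server owning the state.
; Activate runs on authority, calling OpenDoorOnAll and flipping Open, whose OnRep snaps the mesh rotation.
; A timeline scaled by open/close times swings the yaw from its starting rotation, with Pawn collision ignored until it finishes.
; Hovering shows an Open/Close prompt on the player's interact widget.
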(event Custom|OpenDoorOnAll
  (params (Opening :type Boolean))
  (bind _doortimeline (Variables|Default|GetDoorTimeline))
  (bind _baserotation (Variables|Default|GetBaseRotation))
  ;[1 1 1] Ignores Pawn on Open
  (Collision|SetCollisionResponsetoChannel (Variables|Default|GetDoorMesh) "ECC_Pawn" "ECR_Ignore")
  (if Opening
    (Components|Timeline|SetPlayRate _doortimeline (/ 1.0 (Variables|Default|GetTimeToOpen)))
    (bind _alpha (Timeline|DoorTimeline Play)
      (:Update
        (bind _output_get (Variables|Default|SetAlpha _alpha))
        (Transformation|SetRelativeRotation (Variables|Default|GetDoorMesh) (Math|Rotator|MakeRotator 0.0 0.0 (Math|Float|Lerp (.yaw _baserotation) (+ (.yaw _baserotation) (.yaw (Variables|Default|GetOpenRotation))) _output_get)) false false))
      (:Finished
        ;[1 1 1] Ignores Pawn on Open
        (Collision|SetCollisionResponsetoChannel (Variables|Default|GetDoorMesh) "ECC_Pawn" "ECR_Block")))
    (else
      (Components|Timeline|SetPlayRate _doortimeline (/ 1.0 (Variables|Default|GetTimeToClose)))
      (Timeline|DoorTimeline Reverse))))

(event EventBeginPlay
  (|CallParentFunction)
  (Variables|Default|SetBaseRotation (Variables|/Script/Engine.SceneComponent|GetRelativeRotation (Variables|Default|GetDoorMesh))))

(event Collision|EventActorBeginOverlap
  (params (OtherActor :type Actor%20Object%20Reference))
  (|CallParentFunction OtherActor) ; This node is disabled and will not be called.\nDrag off pins to build functionality.
)

(event EventTick
  (params (DeltaSeconds :type Float%20%28single-precision%29))
  (|CallParentFunction DeltaSeconds) ; This node is disabled and will not be called.\nDrag off pins to build functionality.
)

(event EventActivate
  (params (Player%20Controller :type Player%20Controller%20Object%20Reference) (Hit%20Result :type Hit%20Result%20Structure) (Character :type Express%20Lane%20Character%20Object%20Reference))
  (Networking|SwitchHasAuthority
    (:Authority
      (CallFunction|OpenDooronAll (not (Variables|Default|GetOpen?)))
      (Variables|Default|SetOpen? (not (Variables|Default|GetOpen?))))))

(event EventHovered
  (params (Player%20Controller :type Player%20Controller%20Object%20Reference) (Hit%20Result :type Hit%20Result%20Structure) (Character :type Express%20Lane%20Character%20Object%20Reference))
  ;[1 1 1] Event Hovered
  (Variables|/Game/TwentyItems/Blueprints/Player/ExpressLaneCharacter.ExpressLaneCharacter_C|SetWidgetSwitcherIndex Character 1)
  (Variables|/Game/TwentyItems/Blueprints/Player/ExpressLaneCharacter.ExpressLaneCharacter_C|SetHoveredMessage Character (Utilities|Text|FormatText "{Open?} {Text}" (select (Variables|Default|GetOpen?) "Close" "Open") (Variables|Default|GetInteractMessage)))
  (Default|UpdateInteractMessage (Variables|/Game/TwentyItems/Blueprints/Main/PC_ExpressLane.PC_ExpressLane_C|GetInteractMessageWidget (Default|GetPlayerControllerClient Character)) 0 "None"))

(fn ConstructionScript
  (|CallParentFunction))

(fn SetDoorOpen
  (Transformation|SetRelativeRotation (Variables|Default|GetDoorMesh) (select (Variables|Default|GetOpen?) (Variables|Default|GetOpenRotation) "0, 0, 0") false false))

(fn OnRepOpen?
  (CallFunction|SetDoorOpen))

(fn IgnoreOverlappingPlayers
  (Utilities|Array|Clear (Variables|Default|GetOverlappingPlayers))
  (for _array_element (Collision|GetOverlappingActors (Variables|Default|GetDoorMesh) "/Script/Engine.Pawn" :!class /Script/Engine.PrimitiveComponent)
    (Collision|IgnoreActorwhenMoving (Variables|Default|GetDoorMesh) _array_element true)
    (bind _ascharacter (Utilities|Casting|CastToCharacter _array_element))
    (Collision|IgnoreActorwhenMoving (Variables|/Script/Engine.Character|GetCapsuleComponent _ascharacter) _array_element true))
  ;[1 1 1] Ignores Pawn on Open
  (Collision|SetCollisionResponsetoChannel (Variables|Default|GetDoorMesh) "ECC_Pawn" "ECR_Block"))