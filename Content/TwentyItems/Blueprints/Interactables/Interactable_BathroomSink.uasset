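; Bathroom sink with a sensor faucet that fogs its referenced mirrors while running.
; On the server, a sensor overlap turns the faucet on by weighted chance, imitating unreliable real sensors, and a timer shuts it off.
; The replicated faucet state's OnRep spawns or destroys the water sound and particle.
; Tick adds fog to the mirrors over time while the faucet is on.
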(event OnComponentBeginOverlap(Sensor)
  (params (OverlappedComponent :type Primitive%20Component%20Object%20Reference) (OtherActor :type Actor%20Object%20Reference) (OtherComp :type Primitive%20Component%20Object%20Reference) (OtherBodyIndex :type Integer) (bFromSweep :type Boolean) (SweepResult :type Hit%20Result%20Structure%20%28by%20ref%29))
  ;[1 1 1] Event Overlap Sensor
  (Networking|SwitchHasAuthority
    (:Authority
      ;;[0 0.5 1 1 14] Mimmicking the real life annoyingness of sensors by only activating the faucet part of the time
      (if (Math|Random|RandomBoolwithWeight (Variables|Default|GetFaucetActivationRandomWeight))
        ;;[1 1 1] Makes sure the faucet isn't on already
        (if (not (Variables|Default|GetFaucetOn?))
          ;;[1 1 1] Activates the Faucet
          (CallFunction|ActivateFaucet))))))

(event EventBeginPlay
  (|CallParentFunction))

(event Collision|EventActorBeginOverlap
  (params (OtherActor :type Actor%20Object%20Reference))
  (|CallParentFunction OtherActor) ; This node is disabled and will not be called.\nDrag off pins to build functionality.
)

(event EventTick
  (params (DeltaSeconds :type Float%20%28single-precision%29))
  ;[1 1 1] Fogs Up Mirrors When Faucet is on
  (|CallParentFunction DeltaSeconds)
  (if (Variables|Default|GetFaucetOn?)
    (for _array_element (Variables|Default|GetMirrorReferences)
      (Default|AddFogValue _array_element (* DeltaSeconds 1.0)))))

(fn ConstructionScript
  (|CallParentFunction))

(fn OnRepFaucetOn?
  (if (Variables|Default|GetFaucetOn?)
    (CallFunction|Fauceton)
    (else
      (CallFunction|FaucetOff))))

(fn ActivateFaucet
  ;[1 1 1] Sets Faucet On
  (Variables|Default|SetFaucetOn? true)
  ;[1 1 1] Sets Timer To Turn Off Faucet
  (bind _returnvalue (Utilities|Time|SetTimerbyFunctionName 0 "FaucetTimer" (Variables|Default|GetFaucetOnTime)))
  (Variables|Default|SetFaucetTimerHandle _returnvalue))

(fn FaucetOff
  (bind _faucetsoundcomponent (Variables|Default|GetFaucetSoundComponent))
  (bind _faucetparticlecomponent (Variables|Default|GetFaucetParticleComponent))
  (Utilities|FlowControl|Sequence
    (:then_0
      ;[1 0.5 1] Turns off faucet sound
      (Utilities|IsValid _faucetsoundcomponent
        (:Is%20Valid
          (Components|DestroyComponent _faucetsoundcomponent))))
    (:then_1
      ;[1 0.5 1] Destroys Faucet Particle
      (Utilities|IsValid _faucetparticlecomponent
        (:Is%20Valid
          (Components|DestroyComponent _faucetparticlecomponent))))))

(fn Fauceton
  (Utilities|FlowControl|Sequence
    (:then_0
      ;[1 0.5 1] Plays Faucet on Sound
      (if (not (Utilities|IsValid (Variables|Default|GetFaucetSoundComponent)))
        (bind _returnvalue (CallFunction|SpawnSoundatLocationFunction (Variables|Effects|GetFaucetSound) (Transformation|GetWorldLocation (Variables|Default|GetFaucetLocation)) "0, 0, 0" (.AsExpress%20Lane%20Game%20Instance (Utilities|Casting|CastToExpressLane_GameInstance (Game|GetGameInstance))) "NewEnumerator0"))
        (Variables|Default|SetFaucetSoundComponent _returnvalue)))
    (:then_1
      ;[1 0.5 1] Spawns Faucet Particle
      (if (not (Utilities|IsValid (Variables|Default|GetFaucetParticleComponent)))
        (bind _returnvalue_2 (Effects|SpawnEmitteratLocation (Variables|Default|GetFaucetParticle) (Transformation|GetWorldLocation (Variables|Default|GetFaucetLocation)) (Transformation|GetActorRotation)))
        (Variables|Default|SetFaucetParticleComponent _returnvalue_2)))))

(fn FaucetTimer
  (if (Variables|Default|GetFaucetOn?)
    (Variables|Default|SetFaucetOn? false)
    (Utilities|Time|ClearandInvalidateTimerbyHandle (Variables|Default|GetFaucetTimerHandle))))