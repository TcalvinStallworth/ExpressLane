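; Sliding double door that opens when something enters its trigger volume and closes once the trigger is empty.
; Overlap events run only on the authority and respect the Locked flag before calling ActivateDoor.
; ActivateDoor plays or reverses a timeline that slides both panels apart, at a configurable play rate.
; When the timeline finishes, the authority updates the Open state and closes the door if nothing remains inside.
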(event OnComponentBeginOverlap(Trigger)
  (params (OverlappedComponent :type Primitive%20Component%20Object%20Reference) (OtherActor :type Actor%20Object%20Reference) (OtherComp :type Primitive%20Component%20Object%20Reference) (OtherBodyIndex :type Integer) (bFromSweep :type Boolean) (SweepResult :type Hit%20Result%20Structure%20%28by%20ref%29))
  (Networking|SwitchHasAuthority
    (:Authority
      (if (not (Variables|Default|GetLocked?))
        (CallFunction|ActivateDoor true)))))

(event OnComponentEndOverlap(Trigger)
  (params (OverlappedComponent :type Primitive%20Component%20Object%20Reference) (OtherActor :type Actor%20Object%20Reference) (OtherComp :type Primitive%20Component%20Object%20Reference) (OtherBodyIndex :type Integer))
  (Networking|SwitchHasAuthority
    (:Authority
      (if (Math|Boolean|ANDBoolean (Variables|Default|GetOpen?) (== (Utilities|Array|Length (Collision|GetOverlappingActors (Variables|Default|GetTrigger) 0 :!class /Script/Engine.PrimitiveComponent)) 0) (not (Variables|Default|GetLocked?)))
        (CallFunction|ActivateDoor false)))))

(event Custom|ActivateDoor
  (params (Open? :type Boolean))
  (if Open?
    (bind _alpha (Timeline|DoorTimeLine Play)
      (:Update
        (Transformation|SetRelativeLocation (Variables|Default|GetRightDoor) (Math|Vector|Lerp(Vector) "0, 0, 0" "90.000000, 0,0.000000" _alpha) false false)
        (Transformation|SetRelativeLocation (Variables|Default|GetLeftDoor) (Math|Vector|Lerp(Vector) "0, 0, 0" "-90.000000, 0,0.000000" _alpha) false false))
      (:Finished
        (Networking|SwitchHasAuthority
          (:Authority
            (Variables|Default|SetOpen? Open?)
            (if (not (> (Utilities|Array|Length (Collision|GetOverlappingActors (Variables|Default|GetTrigger) 0 :!class /Script/Engine.PrimitiveComponent)) 0))
              (CallFunction|ActivateDoor false))))))
    (else
      (Timeline|DoorTimeLine Reverse))))

(event EventBeginPlay
  (|CallParentFunction)
  ;[1 1 1] How long it takes to open the doors
  (Components|Timeline|SetPlayRate (Variables|Default|GetDoorTimeLine) (Variables|Default|GetTimelinePlayRate)))

(event Collision|EventActorBeginOverlap
  (params (OtherActor :type Actor%20Object%20Reference))
  (|CallParentFunction OtherActor) ; This node is disabled and will not be called.\nDrag off pins to build functionality.
)

(event EventTick
  (params (DeltaSeconds :type Float%20%28single-precision%29))
  (|CallParentFunction DeltaSeconds))

(fn ConstructionScript
  (|CallParentFunction))