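; Bombay is a team's placeable, destructible spawn point that doubles as an item store.
; On begin play the server registers it with the team, loads health from data and fills stock from fixed items plus weighted random picks.
; Activation opens a team-checked store widget; purchases route through the player controller, charge money and spawn items.
; Non-friendly damage can destroy it, flagging the team; grace-period immunity and stock forfeiture are unwired.
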(event Custom|PlayBombayTakeDamageEffects)

(event Custom|PlayBombayDestroyedEffects
  (bind _returnvalue (Transformation|GetActorTransform))
  (bind _returnvalue_2 (Transformation|GetActorTransform))
  ;[1 0.5 1] Play Bombay Destroyed Effects
  (Effects|SpawnEmitteratLocation (Variables|Effects|GetBombayDestroyedEmitter) (.location _returnvalue_2) (.rotation _returnvalue_2) (.scale _returnvalue_2))
  (CallFunction|PlaySoundatLocationFunction (Variables|Effects|GetBombayDestroyedSound) (.location _returnvalue) (.rotation _returnvalue) (.AsExpress%20Lane%20Game%20Instance (Utilities|Casting|CastToExpressLane_GameInstance (Game|GetGameInstance))) "NewEnumerator0"))

(event Custom|AttemptPurchaseItem
  (params (Index :type Integer) (Character :type Express%20Lane%20Character%20Object%20Reference))
  ;[1 1 1] Attempt Purchase Item
  (Purchasing|AttemptPurchaseItemFunction Index Character))

(event EventBeginPlay
  ;[1 0 0] Event Begin Play
  (Networking|SwitchHasAuthority
    (:Authority
      (CallFunction|UpdateOwningTeam)
      (CallFunction|RemoveBombayTrapsfromTeam)
      (Health|InitiateBombayHealth)
      (Store|CreateStore)
      (CallFunction|AddOwningTeamtoRoster)
      (Default|AddBombaytoMap (Variables|Default|GetOwningTeam)))))

(event EventDealDamage
  (params (Damage :type Integer) (Controller :type Controller%20Object%20Reference) (Weapon :type Actor%20Object%20Reference) (Blockable :type Boolean) (Hit%20Result :type Hit%20Result%20Structure) (AttackID :type Integer))
  ;[1 1 1] Damage Function
  (Networking|SwitchHasAuthority
    (:Authority
      (Health|BombayDamageFunction Damage Controller Weapon Blockable Hit%20Result AttackID))))

(event EventActivate
  (params (Player%20Controller :type Player%20Controller%20Object%20Reference) (Hit%20Result :type Hit%20Result%20Structure) (Character :type Express%20Lane%20Character%20Object%20Reference))
  ;[1 1 1] Event Activate
  (Store|AttemptInteract Player%20Controller Hit%20Result Character))

(event EventUpdateOwningTeam
  (if (Utilities|Array|ContainsItem (Variables|/Game/TwentyItems/Blueprints/Main/Skylands/TeamManager.TeamManager_C|GetMembers (Variables|Default|GetOwningTeam)) (.AsPS%20Express%20Lane (Utilities|Casting|CastToPS_ExpressLane (Variables|/Script/Engine.Controller|GetPlayerState (Game|GetPlayerController 0)))))
    (Development|SetHiddeninGame (Variables|Default|GetBeacon) false false)))

(event Custom|PlayPurchaseEffects
  (bind _itemspawnlocation (Variables|Default|GetItemSpawnLocation))
  (CallFunction|PlaySoundatLocationFunction (Variables|Effects|GetPurchaseSound) (Transformation|GetWorldLocation _itemspawnlocation) (Transformation|GetWorldRotation _itemspawnlocation) (.AsExpress%20Lane%20Game%20Instance (Utilities|Casting|CastToExpressLane_GameInstance (Game|GetGameInstance))) "NewEnumerator0"))

(fn ConstructionScript)

(fn GetGameModeRef
  (Networking|SwitchHasAuthority
    (:Authority
      (Utilities|IsValid (Variables|References|GetGM%20Skylands)
        (:Is%20Valid
          _)
        (:Is%20Not%20Valid
          (Variables|References|SetGM%20Skylands (.AsGM%20Skylands (Utilities|Casting|CastToGM_Skylands (Game|GetGameMode))))))
      (return (Variables|References|GetGM%20Skylands)))))

(fn InitiateBombayHealth
  (Networking|SwitchHasAuthority
    (:Authority
      ;[1 1 1] Sets Bombay's initial health
      (bind _output_get (Variables|Default|SetMaxHealth (.MaxHealth (Utilities|Struct|BreakTrapParametersStruct (.Data (CallFunction|GetTrapParametersDatafromDataTable (Variables|Default|GetDataKey)))))))
      (Variables|Default|SetHealth _output_get))))

(fn BombayDamageFunction
  (params (Damage :type Integer) (Controller :type Controller%20Object%20Reference) (Weapon :type Actor%20Object%20Reference) (Blockable :type Boolean) (Hit%20Result :type Hit%20Result%20Structure) (AttackID :type Integer))
  (Networking|SwitchHasAuthority
    (:Authority
      (LocalVariables|SetDamage%20 Damage)
      (LocalVariables|SetController%20 Controller)
      (LocalVariables|SetWeapon%20 Weapon)
      (LocalVariables|SetHit%20Result%20 Hit%20Result)
      ;[1 1 1] Bombays are immune to damage in Grace Period
      (if (not (Variables|/Game/TwentyItems/Blueprints/Main/Testing/Servertesting/ServerGameMode.ServerGameMode_C|GetBombaysInvulnerable? (.AsServer%20Game%20Mode (Utilities|Casting|CastToServerGameMode (Game|GetGameMode)))))
        _
        (else
          _))
      ;[1 1 1] Makes sure its not friendly fire
      (if (not (Utilities|Array|ContainsItem (Variables|/Game/TwentyItems/Blueprints/Main/Skylands/TeamManager.TeamManager_C|GetMembers (Variables|Default|GetOwningTeam)) (.AsPS%20Express%20Lane (Utilities|Casting|CastToPS_ExpressLane (Variables|/Script/Engine.Controller|GetPlayerState (LocalVariables|GetController%20))))))
        ;[0 0 0] Subtracts Health
        (bind _output_get (Variables|Default|SetHealth (- (Variables|Default|GetHealth) (LocalVariables|GetDamage%20))))
        ;[1 1 1] Checks if the bombay has been destroyed
        (if (<= _output_get 0)
          ;[1 1 1] Sets Bombay Destroyed to True
          (Variables|/Game/TwentyItems/Blueprints/Main/Skylands/TeamManager.TeamManager_C|SetBombayDestroyed? (Variables|Default|GetOwningTeam) true)
          ;[1 1 1] Plays Effects on Clients
          (CallFunction|PlayBombayDestroyedEffects)
          (Utilities|FlowControl|Sequence
            (:then_1
              (Store|ForfeitStoreStock (LocalVariables|GetController%20))
              (Utilities|FlowControl|Sequence
                (:then_0
                  (if (CallFunction|ClassEqual? (LocalVariables|GetController%20) "/Game/TwentyItems/Blueprints/Main/Skylands/PC_ExpressLane.PC_ExpressLane_C")
                    (Default|SendTeamMessage (Variables|Default|GetOwningTeam) (Utilities|Text|FormatText "{Player} Destroyed Your Spawn Point!" (Variables|/Game/TwentyItems/Blueprints/Main/Skylands/PS_ExpressLane.PS_ExpressLane_C|GetUsernameExpresslane (Default|GetPlayerStateRef (.AsPC%20Express%20Lane (Utilities|Casting|CastToPC_ExpressLane (LocalVariables|GetController%20)))))) "(R=1.000000,G=1.000000,B=1.000000,A=1.000000)" 5.0)))
                (:then_1
                  ;[1 1 1] Destroys Bombay
                  (Actor|DestroyActor)))))
          (else
            (UI|BombayBeingAttackedMessage)))))))

(fn OnRepWeaponStock)

(fn OnRepConsumableStock)

(fn OnRepAmmoStock)

(fn CreateStore
  (Networking|SwitchHasAuthority
    (:Authority
      (Store|AddAlwaysSpawnedItems)
      (Store|SelectSpawnedItems (Utilities|Array|MakeArray "NewEnumerator0" "NewEnumerator2") (Variables|Store|GetWeaponStockRange))
      (Store|SelectSpawnedItems (Utilities|Array|MakeArray "NewEnumerator1" "NewEnumerator3" "NewEnumerator5") (Variables|Store|GetConsumableStockRange))
      (Store|SelectSpawnedItems (Utilities|Array|MakeArray "NewEnumerator4") (Variables|Store|GetAmmoStockRange)))))

(fn AddAlwaysSpawnedItems
  (Utilities|Array|AppendArray (Variables|Store|GetStoreStock) (.Loot (Utilities|Struct|BreakLootContainerStruct (.Data (CallFunction|GetSpawnableLootContainerDatafromDataTable "BombayStoreAlwaysSpawned"))))))

(fn ContainsItem?
  (params (Item%20Key :type Name))
  (LocalVariables|SetItem%20 Item%20Key)
  (bind (_array_element _array_index) (Utilities|Array|ForEachLoopwithBreak (Variables|Store|GetStoreStock) :!label _label)
    (:LoopBody
      (if (Utilities|Name|Equal(Name) (.DataKey (Utilities|Struct|BreakLootable_Struct _array_element)) (LocalVariables|GetItem%20))
        (LocalVariables|SetContains? true)
        (LocalVariables|SetIndex%20 _array_index)
        (goto _label Break)
        (else
          (LocalVariables|SetContains? false))))
    (:Completed
      (return (LocalVariables|GetContains?) (LocalVariables|GetIndex%20)))))

(fn AttemptPurchaseItemClient
  (params (Data%20Key :type Name))
  (bind (__return _index) (Store|ContainsItem? Data%20Key))
  (LocalVariables|SetItem%20Key Data%20Key)
  (if __return
    (if (Default|CanPlayerAfford (Default|GetPlayerStateRef (.AsExpress%20Lane%20Character (Utilities|Casting|CastToExpressLaneCharacter (Game|GetPlayerCharacter 0)))) (Utilities|Struct|BreakEquippableInventoryStruct (.Data (CallFunction|GetEquippableDatafromTable Data%20Key))))
      (Default|PassPurchasetoServer (.AsPC%20Express%20Lane (Utilities|Casting|CastToPC_ExpressLane (Game|GetPlayerController 0))) _index self))))

(fn AttemptPurchaseItemFunction
  (params (Index :type Integer) (Character :type Express%20Lane%20Character%20Object%20Reference))
  (LocalVariables|SetIndexRef Index)
  (LocalVariables|SetCharacterRef Character)
  (Networking|SwitchHasAuthority
    (:Authority
      ;[1 1 1] Team Check
      (if (or (== (Default|GetTeamReference (Default|GetPlayerStateRef (LocalVariables|GetCharacterRef))) (Variables|Default|GetOwningTeam)) (not (Variables|Store|GetCheckTeam)))
        ;[1 1 1] Checks if the index is valid
        (if (<= (LocalVariables|GetIndexRef) (Utilities|Array|LastIndex (Variables|Store|GetStoreStock)))
          ;[1 1 1] Checks if player can afford the Item
          (if (Default|CanPlayerAfford (Default|GetPlayerStateRef (LocalVariables|GetCharacterRef)) (.Price (Utilities|Struct|BreakEquippableInventoryStruct (.Data (CallFunction|GetEquippableDatafromTable (.DataKey (Utilities|Struct|BreakLootable_Struct (Utilities|Array|Get(acopy) (Variables|Store|GetStoreStock) (LocalVariables|GetIndexRef)))))))))
            ;[0 0 0] Pays for Product
            (Default|RemovePlayerMoney (Default|GetPlayerStateRef (LocalVariables|GetCharacterRef)) (.Price (Utilities|Struct|BreakEquippableInventoryStruct (.Data (CallFunction|GetEquippableDatafromTable (.DataKey (Utilities|Struct|BreakLootable_Struct (Utilities|Array|Get(acopy) (Variables|Store|GetStoreStock) (LocalVariables|GetIndexRef)))))))) false)
            ;[1 1 1] SpawnsItem
            (Game|SpawnActorfromClass (.Actor (Utilities|Struct|BreakLootable_Struct (Utilities|Array|Get(acopy) (Variables|Store|GetStoreStock) (LocalVariables|GetIndexRef)))) (Transformation|GetWorldTransform (Variables|Default|GetItemSpawnLocation)) "AdjustIfPossibleButAlwaysSpawn" 0 0)
            (CallFunction|PlayPurchaseEffects)))))))

(fn AttemptInteract
  (params (Player%20Controller :type Player%20Controller%20Object%20Reference) (Hit%20Result :type Hit%20Result%20Structure) (Character :type Express%20Lane%20Character%20Object%20Reference))
  (Networking|SwitchHasAuthority
    (:Authority
      ;[1 1 1] Makes sure the interacting player owns the bombay
      (if (or (== (Default|GetTeamReference (Default|GetPlayerStateRef Character)) (Variables|Default|GetOwningTeam)) (not (Variables|Store|GetCheckTeam)))
        ;[1 1 1] Creates Store Widget
        (Default|CreateBombayStoreWidget (.AsPC%20Express%20Lane (Utilities|Casting|CastToPC_ExpressLane Player%20Controller)) self)))))

(fn ForfeitStoreStock
  (params (Controller :type Controller%20Object%20Reference))
  (LocalVariables|SetControllerRef Controller)
  (Networking|SwitchHasAuthority
    (:Authority
      ;[1 1 1] Checks if the Base was destroyed by a player
      (if (Utilities|ClassIsChildOf (Utilities|GetClass Controller) "/Game/TwentyItems/Blueprints/Main/Skylands/PC_ExpressLane.PC_ExpressLane_C")
        _))))

(fn SelectSpawnedItems
  (params (Item%20Types :type Array%20of%20ItemType%20Enums :default "NewEnumerator0") (Item%20Range :type Dimensions%20Struct%20Structure))
  (bind (_x _y) (Utilities|Struct|BreakDimensionsStruct Item%20Range))
  (Networking|SwitchHasAuthority
    (:Authority
      (LocalVariables|SetItemRange Item%20Range)
      ;[1 1 1] Finds Items matching item types and tallies them up
      (bind (_matching_structs _tallies) (CallFunction|FilterSpawnableLootbyItemTypes "BombayStore" Item%20Types))
      (LocalVariables|SetItemArray _matching_structs)
      (LocalVariables|SetArrayTotalSpawnTallies _tallies)
      ;[0 0.5 1] Selects the number of items spawned
      (bind _output_get (LocalVariables|SetItemsSpawned (Math|Random|RandomIntegerinRange _x _y)))
      (for _index (range 0 (- _output_get 1))
        ;[1 1 1] Selects the Ticket to spawn the Item
        (LocalVariables|SetSpawnedIndex (Math|Random|RandomIntegerinRange 0 (LocalVariables|GetArrayTotalSpawnTallies)))
        ;[1 1 1] Finds Item to Spawn
        (bind (_array_element _array_index) (Utilities|Array|ForEachLoopwithBreak (LocalVariables|GetItemArray) :!label _label)
          (:LoopBody
            (LocalVariables|SetCurrentIndex _array_element)
            (bind _output_get_2 (LocalVariables|SetSelectionAddition (+ (.SpawnRate (Utilities|Struct|BreakLootable_Struct _array_element)) (LocalVariables|GetSelectionAddition))))
            (if (not (> (LocalVariables|GetSpawnedIndex) _output_get_2))
              (Utilities|FlowControl|Sequence
                (:then_0
                  (Utilities|Array|RemoveIndex (LocalVariables|GetItemArray) _array_index)
                  (Utilities|Array|Add (Variables|Store|GetStoreStock) (LocalVariables|GetCurrentIndex)))
                (:then_1
                  (goto _label Break))))))))))

(fn RemoveBombayTrapsfromTeam
  (Networking|SwitchHasAuthority
    (:Authority
      (for _array_element (Variables|/Game/TwentyItems/Blueprints/Main/Skylands/TeamManager.TeamManager_C|GetMembers (Variables|Default|GetOwningTeam))
        (Default|RemovePlayerTrap _array_element "Bombay" 1 true)))))

(fn CreateTeamBombayReference
  (Networking|SwitchHasAuthority
    (:Authority
      (Variables|/Game/TwentyItems/Blueprints/Main/Skylands/TeamManager.TeamManager_C|SetRespawnPointReference (Variables|Default|GetOwningTeam) 0 self))))

(fn AddOwningTeamtoRoster
  (bind _owningteam (Variables|Default|GetOwningTeam))
  (Networking|SwitchHasAuthority
    (:Authority
      (if (Utilities|IsValid (.RespawnPointReference (Variables|/Game/TwentyItems/Blueprints/Main/Skylands/TeamManager.TeamManager_C|GetRespawnPointReference (Variables|Default|GetOwningTeam))))
        (Actor|DestroyActor)
        (else
          (Variables|/Game/TwentyItems/Blueprints/Main/Skylands/TeamManager.TeamManager_C|SetRespawnPointReference _owningteam 0 self)
          (Variables|/Game/TwentyItems/Blueprints/Main/Skylands/TeamManager.TeamManager_C|SetHasBombayBeenPlaced? _owningteam true)
          (Variables|/Game/TwentyItems/Blueprints/Main/Skylands/TeamManager.TeamManager_C|SetBombayDestroyed? _owningteam false))))))

(fn GetGameStateRef
  (Utilities|IsValid (Variables|References|GetGS%20Skylands)
    (:Is%20Valid
      _)
    (:Is%20Not%20Valid
      (bind _output_get (Variables|References|SetGS%20Skylands (.AsGS%20Skylands (Utilities|Casting|CastToGS_Skylands (Game|GetGameState)))))))
  (return _output_get))

(fn BombayBeingAttackedCoolDownMessageTimer
  (Variables|UI|SetBombayBeingAttackedMessageSendable? false))

(fn BombayBeingAttackedMessage
  (params (Attacking%20Controller :type Controller%20Object%20Reference))
  (if (Variables|UI|GetBombayBeingAttackedMessageSendable?)
    (Variables|UI|SetBombayBeingAttackedMessageSendable? false)
    (bind _returnvalue (Utilities|Time|SetTimerbyFunctionName 0 "BombayBeingAttackedCoolDownMessageTimer" 5.0))
    (Variables|UI|SetBombayBeingAttackedCoolDownMessageTimerHandle _returnvalue)))